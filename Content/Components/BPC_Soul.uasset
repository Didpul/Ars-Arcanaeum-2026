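; Soul component that manages its owner's Soul Stability resource and the absorbing of soul orbs and broken enemies.
; Stability changes update the owner's soul state; spending while unstable instead splits the cost between stability and health via a cast callback.
; A looping timer regenerates stability after a retriggerable delay, slower when unstable.
; Absorbing spawns a Niagara vortex and sphere-traces for targets, locking them through interface messages until cancelled.
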(event Custom|Start%20Absorbing
  (bind _returnvalue (Components|GetOwner))
  (bind _returnvalue_2 (Components|GetOwner))
  (bind _returnvalue_3 (Transformation|GetActorLocation _returnvalue))
  (CallFunction|StartVortex)
  (Variables|Default|SetIs%20Absorbing true)
  (bind _outhits (Collision|MultiSphereTraceForObjects _returnvalue_3 _returnvalue_3 1.5e+03 (Utilities|Array|MakeArray "ObjectTypeQuery2" "ObjectTypeQuery3") false 0 "ForOneFrame"))
  (for _array_element _outhits
    (if (Utilities|DoesObjectImplementInterface (.HitActor (Collision|BreakHitResult _array_element)) "/Game/Interfaces/BPI_SoulActor.BPI_SoulActor_C")
      (if (or (== (Utilities|GetClass (.HitActor (Collision|BreakHitResult _array_element))) "/Game/Characters/Soul_Orbs/BP_SoulOrb.BP_SoulOrb_C") (== (Utilities|GetClass (.HitActor (Collision|BreakHitResult _array_element))) "/Game/Characters/Soul_Orbs/BP_HealthOrb.BP_HealthOrb_C"))
        (Utilities|Array|AddUnique (Variables|Default|GetOrbs%20Absorbing) (.HitActor (Collision|BreakHitResult _array_element)))
        (Class|BPISoulActor|LockAbsorber(Message) (.HitActor (Collision|BreakHitResult _array_element)) _returnvalue_2)
        (else
          (bind _combat_comp (Class|BPIDamageable|GetCombatComp(Message) (.HitActor (Collision|BreakHitResult _array_element))))
          (if (Variables|/Game/Components/BpC_Combat.BpC_Combat_C|GetBroken _combat_comp)
            (Class|BPISoulActor|LockAbsorber(Message) (.HitActor (Collision|BreakHitResult _array_element)) _returnvalue_2)
            (Utilities|Array|AddUnique (Variables|Default|GetEnemies%20Absorbing) (.HitActor (Collision|BreakHitResult _array_element)))))))))

(event Custom|Stop%20Absorbing
  (CallFunction|DestroyVfx)
  (Utilities|FlowControl|Sequence
    (:then_0
      (for _array_element (Variables|Default|GetOrbs%20Absorbing)
        (Utilities|IsValid _array_element
          (:Is%20Valid
            (Class|BPISoulActor|CancelAbsorb(Message) _array_element)))))
    (:then_1
      (for _array_element_2 (Variables|Default|GetEnemies%20Absorbing)
        (Utilities|IsValid _array_element_2
          (:Is%20Valid
            (Class|BPISoulActor|CancelAbsorb(Message) _array_element_2)))))))

(event Custom|Start%20Vortex
  (bind _returnvalue (Components|GetOwner))
  (bind _returnvalue_2 (Actor|GetComponentbyClass _returnvalue "/Script/Engine.SkeletalMeshComponent"))
  (Utilities|FlowControl|DoOnce false
    (:Completed
      (bind _returnvalue_3 (Niagara|SpawnSystemAttached "/Game/Art/NFX_Vortex.NFX_Vortex" _returnvalue_2 (Transformation|GetAttachSocketName _returnvalue_2) (Transformation|GetActorLocation _returnvalue) "0, 0, 0" "SnapToTargetIncludingScale" false))
      (Variables|Default|Setvortex _returnvalue_3)
      (Transformation|DetachFromComponent _returnvalue_3 "KeepRelative" "KeepRelative" "KeepRelative" true)
      (Transformation|AttachComponentToComponent _returnvalue_3 _returnvalue_2 "ROOT" "SnapToTarget" "SnapToTarget" "SnapToTarget" true))))

(event Custom|Destroy%20vfx
  (Components|DestroyComponent (Variables|Default|Getvortex))
  (CallFunction|ResetVortex))

(event Custom|reset%20vortex
  (bind _returnvalue (Components|GetOwner))
  (bind _returnvalue_2 (Actor|GetComponentbyClass _returnvalue "/Script/Engine.SkeletalMeshComponent"))
  (Utilities|FlowControl|DoOnce false) ; enters at Reset
)

(event Custom|Recover%20Over%20time
  (bind _returnvalue (Utilities|Time|SetTimerbyEvent (delegate Custom|start%20recovering) 0.1 true))
  (Variables|Default|SetRegenHandle _returnvalue))

(event Custom|start%20recovering
  (if (>= (Variables|Default|GetSoulStability) (Variables|Default|GetMaxSoulStability))
    (Utilities|Time|ClearandInvalidateTimerbyHandle (Variables|Default|GetRegenHandle))
    (else
      (CallFunction|ModifyStability (Math|Float|SelectFloat 0.5 1.0 (Variables|Default|GetIsUnstable)) true))))

(event Custom|stop%20regen
  (if (Utilities|Time|IsValidTimerHandle (Variables|Default|GetRegenHandle))
    (Utilities|Time|ClearandInvalidateTimerbyHandle (Variables|Default|GetRegenHandle)))
  ;[1 1 1] Time before regen starts again
  (Utilities|FlowControl|RetriggerableDelay 2.0)
  (CallFunction|RecoverOverTime))

(fn ModifyStability
  (params (Amount :type Float%20%28double-precision%29) (Add :type Boolean))
  (if Add
    (Variables|Default|SetSoulStability (Math|Float|Clamp(Float) (+ (Variables|Default|GetSoulStability) Amount) 0.0 (Variables|Default|GetMaxSoulStability)))
    (CallFunction|CheckUnstable :!label _label)
    (Default|CallStabilityUpdated)
    (return (Variables|Default|GetSoulStability))
    (elif (not (Variables|Default|GetIsUnstable))
      (Variables|Default|SetSoulStability (Math|Float|Clamp(Float) (- (Variables|Default|GetSoulStability) Amount) 0.0 (Variables|Default|GetMaxSoulStability)))
      (goto _label)
      (else
        (CallFunction|UnstableCast Amount)))))

(fn CheckUnstable
  (if (not (Variables|Default|GetIsUnstable))
    (if (<= (Variables|Default|GetSoulStability) (Variables|Default|GetDangerZone))
      (if (<= (Variables|Default|GetSoulStability) 0.0)
        (Variables|Default|SetIsUnstable true)
        (Class|BPIPlayer|ChangeSoulState(Message) (Components|GetOwner) "NewEnumerator2")
        (else
          (Class|BPIPlayer|ChangeSoulState(Message) (Components|GetOwner) "NewEnumerator1")))
      (else
        (Variables|Default|SetIsUnstable false)
        (Class|BPIPlayer|ChangeSoulState(Message) (Components|GetOwner) "NewEnumerator0")))))

(fn UnstableCast
  (params (Full%20Amount :type Float%20%28double-precision%29))
  (bind _soulstability (Variables|Default|GetSoulStability))
  (bind _returnvalue (Math|Float|Min(Float) _soulstability Full%20Amount))
  (Default|CallOnUnstableCast _returnvalue (- Full%20Amount _returnvalue)))

(fn SubstractStability
  (params (Stab%20to%20Subs :type Float%20%28double-precision%29))
  (Variables|Default|SetSoulStability (Math|Float|Clamp(Float) (- (Variables|Default|GetSoulStability) Stab%20to%20Subs) 0.0 (Variables|Default|GetMaxSoulStability)))
  (Default|CallStabilityUpdated))