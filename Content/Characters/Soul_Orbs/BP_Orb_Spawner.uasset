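; BP_Orb_Spawner is a spawner actor that keeps one orb of a configurable class present at its location.
; A looping two-second timer started on BeginPlay checks the last spawned actor and spawns a replacement slightly above the spawner once that reference is invalid.
; The construction script passes a Color variable to the Niagara component to tint its effect.
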(event Custom|Spawn%20check
  (Utilities|IsValid (Variables|Default|GetSpawned%20actor)
    (:Is%20Not%20Valid
      (CallFunction|SpawnORb))))

(event Custom|Spawn%20ORb
  (bind _returnvalue (Game|SpawnActorfromClass (Variables|Default|GetClass) (Math|Transform|MakeTransform (+ (Transformation|GetActorLocation) "0.000000,0.000000,50.000000")) "Undefined" "MultiplyWithRoot" 0 0))
  (Variables|Default|SetSpawned%20actor _returnvalue))

(event EventBeginPlay
  (Utilities|Time|SetTimerbyEvent (delegate Custom|Spawn%20check) 2.0 true))

(fn ConstructionScript
  (Niagara|SetNiagaraVariable(LinearColor) (Variables|Default|GetNiagara) "Color" (Variables|Default|GetColor)))