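; Combat component that gives its owning actor melee hit detection, health, damage reactions and soft lock.
; Socket sphere traces damage each non-team pawn once through interface messages, with hitstop via custom time dilation.
; DamageReceived checks immunity, block and pierce, then breaks, kills, or runs the ReactionChecker macro for profile-driven montage, knockback, hitstop and turning.
; Soft lock faces a nearby pawn, held by a retriggerable delay; helpers handle healing and material flashes.
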(event Custom|MatFlash2nd
  (params (Mat :type Material%20Instance%20Dynamic%20Object%20Reference) (bPickA :type Boolean) (A :type Linear%20Color%20Structure))
  ;[1 1 1] MatFlash
  (Rendering|Material|SetVectorParameterValue Mat "Flash Color" (Math|Color|SelectColor A "(R=1.000000,G=1.000000,B=1.000000,A=1.000000)" bPickA) :!class /Script/Engine.MaterialInstanceDynamic)
  (Rendering|Material|SetScalarParameterValue Mat "Flash" 1.0 :!class /Script/Engine.MaterialInstanceDynamic)
  (Utilities|FlowControl|Delay 0.2)
  (Rendering|Material|SetScalarParameterValue Mat "Flash" 0.0 :!class /Script/Engine.MaterialInstanceDynamic))

(event Custom|Hitstop
  (params (Actor :type Actor%20Object%20Reference) (Slow/Stop :type Boolean))
  ;[0.2808 0.2626 0.3958 1 50] Hitstop
  (Variables|/Script/Engine.Actor|SetCustomTimeDilation Actor (Math|Float|SelectFloat 0.25 0.0 Slow/Stop))
  (Utilities|FlowControl|Delay 0.15)
  (Variables|/Script/Engine.Actor|SetCustomTimeDilation Actor 1.0))

(event Custom|Sphere%20trace
  (params (Target :type Scene%20Component%20Object%20Reference) (InSocketName :type Name) (Radius :type Float%20%28single-precision%29) (Damage%20Profile :type PDA%20Damage%20Profile%20Object%20Reference))
  (bind _returnvalue (Transformation|GetSocketLocation Target InSocketName))
  (bind _returnvalue_2 (Components|GetOwner))
  ;[0.2808 0.2626 0.3958 1 50] Basic trace
  (Variables|Default|SetDamage%20Profile Damage%20Profile)
  (bind (_outhits _returnvalue_3) (Collision|MultiSphereTraceForObjects _returnvalue _returnvalue Radius (Utilities|Array|MakeArray "ObjectTypeQuery3") false 0 "None"))
  (for _array_element _outhits
    (if _returnvalue_3
      (bind _team_number (Class|BPIDamageable|GetTeamNumber(Message) (.HitActor (Collision|BreakHitResult _array_element))))
      (if (not (== _team_number (Variables|Default|GetTeam%20number)))
        (if (not (Utilities|Array|ContainsItem (Variables|Default|GetDamaged%20Enemies) (.HitActor (Collision|BreakHitResult _array_element))))
          (CallFunction|Hitstop _returnvalue_2 false)
          (Class|BPIDamageable|ReceiveDamage(Message) (.HitActor (Collision|BreakHitResult _array_element)) _returnvalue_2 (Utilities|Struct|MakeS_DamageInfo 1e+01 "NewEnumerator0" "NewEnumerator0" (Variables|Default|GetDamage%20Profile)))
          (Utilities|Array|AddUnique (Variables|Default|GetDamaged%20Enemies) (.HitActor (Collision|BreakHitResult _array_element)))
          (Default|CallMeleeHit))))))

(event Custom|Soft%20lock
  (bind _returnvalue (Components|GetOwner))
  (bind _returnvalue_2 (Components|GetOwner))
  (bind _returnvalue_3 (Transformation|GetActorLocation _returnvalue))
  ;[0.2808 0.2626 0.3958 1 50] Soft lock
  (Variables|Default|GetGlued%20Actor
    (:then
      (Transformation|SetActorRotation _returnvalue_2 (Math|Rotator|MakeRotator 0.0 0.0 (.yaw (Math|Rotator|FindLookatRotation (Transformation|GetActorLocation _returnvalue_2) (Transformation|GetActorLocation (Variables|Default|GetGlued%20Actor))))) :!label _label)
      (Utilities|FlowControl|RetriggerableDelay 1.0)
      (Variables|Default|SetGlued%20Actor 0))
    (:else
      (bind (_outhits _returnvalue_4) (Collision|MultiSphereTraceForObjects _returnvalue_3 _returnvalue_3 1.5e+02 (Utilities|Array|MakeArray "ObjectTypeQuery3") false 0 "None" true "(R=1.000000,G=0.000000,B=0.000000,A=1.000000)" "(R=0.000000,G=1.000000,B=0.000000,A=1.000000)" 2.0))
      (if _returnvalue_4
        (Variables|Default|SetGlued%20Actor (.HitActor (Collision|BreakHitResult (Utilities|Array|Get(acopy) _outhits))))
        (goto _label)))))

(event Custom|MatFlash
  (params (Mat :type Material%20Instance%20Dynamic%20Object%20Reference) (Alter%20Color :type Boolean) (Color :type Linear%20Color%20Structure))
  ;[1 1 1] MatFlash
  (Rendering|Material|SetVectorParameterValue Mat "Flash Color" (Math|Color|SelectColor Color "(R=1.000000,G=1.000000,B=1.000000,A=1.000000)" Alter%20Color) :!class /Script/Engine.MaterialInstanceDynamic)
  (Rendering|Material|SetScalarParameterValue Mat "Flash" 1.0 :!class /Script/Engine.MaterialInstanceDynamic)
  (Utilities|FlowControl|Delay 0.2)
  (Rendering|Material|SetScalarParameterValue Mat "Flash" 0.0 :!class /Script/Engine.MaterialInstanceDynamic))

(event EventBeginPlay)

(event EventTick
  (params (DeltaSeconds :type Float%20%28single-precision%29)))

(fn DamageReceived
  (params (Damage%20causer :type Actor%20Object%20Reference) (Dmg%20Info :type S%20Damage%20Info%20Structure))
  (bind (_amount _damagetype _effects _damageprofile) (Utilities|Struct|BreakS_DamageInfo Dmg%20Info))
  (bind (_amount_2 _damagetype_2 _effects_2 _damageprofile_2) (Utilities|Struct|BreakS_DamageInfo Dmg%20Info))
  (bind _returnvalue (Components|GetOwner))
  (bind _returnvalue_2 (Components|GetOwner))
  (if (not (Variables|Default|GetImmune))
    (if (Variables|Default|GetBlock)
      (if (Variables|/Game/Core/Damage/PDA_DamageProfile.PDA_DamageProfile_C|GetPierce _damageprofile)
        (if (not (Variables|Default|GetBroken)) :!label _label
          (bind _output_get (Variables|Default|SetHealth (- (Variables|Default|GetHealth) _amount)))
          (if (<= _output_get 0.0)
            (if (Variables|Default|GetIsBreakable?)
              (if (not (Variables|Default|GetBroken))
                (Variables|Default|SetBroken true)
                (Class|BPIDamageable|Break(Message) _returnvalue))
              (else
                (Class|BPIDamageable|Die(Message) _returnvalue false)))
            (else
              (switch Utilities|FlowControl|Switch|SwitchonE_DamageTypes _damagetype_2
                (:NewEnumerator0
                  _)
                (:NewEnumerator1
                  (Default|CallSpellHit)))
              (Utilities|ReactionChecker (Variables|/Game/Core/Damage/PDA_DamageProfile.PDA_DamageProfile_C|GetPlay%20Montage _damageprofile_2) (Variables|/Game/Core/Damage/PDA_DamageProfile.PDA_DamageProfile_C|GetKnockback _damageprofile_2) (Variables|/Game/Core/Damage/PDA_DamageProfile.PDA_DamageProfile_C|GetHitstop _damageprofile_2) (Variables|/Game/Core/Damage/PDA_DamageProfile.PDA_DamageProfile_C|GetRotate _damageprofile_2)
                (:play
                  (Class|BPIDamageable|DamageReaction(Message) (Components|GetOwner) Damage%20causer _damagetype_2))
                (:back
                  (bind _ascharacter (Utilities|Casting|CastToCharacter _returnvalue_2))
                  (Reactions|Knockback _ascharacter Damage%20causer))
                (:hit
                  (CallFunction|Hitstop _returnvalue_2 false))
                (:tation
                  (Reactions|Rotate Damage%20causer)))))
          (else
            (switch Utilities|FlowControl|Switch|SwitchonE_DamageTypes _damagetype
              (:NewEnumerator0
                (Default|CallOnBrokenHit))
              (:NewEnumerator1
                (Default|CallSpellHit)))))
        (else
          (Default|CallOnBlock Damage%20causer)))
      (else
        (goto _label)))))

(fn Rotate
  (params (Causer :type Actor%20Object%20Reference))
  (bind _returnvalue (Components|GetOwner))
  (Transformation|SetActorRotation _returnvalue (Math|Rotator|MakeRotator 0.0 0.0 (.yaw (Math|Rotator|FindLookatRotation (Transformation|GetActorLocation _returnvalue) (Transformation|GetActorLocation Causer))))))

(fn Knockback
  (params (Affected :type Character%20Object%20Reference) (Causer :type Actor%20Object%20Reference))
  (bind _returnvalue (Transformation|GetActorLocation Affected))
  (bind _returnvalue_2 (Transformation|GetActorLocation Causer))
  (bind _returnvalue_3 (- _returnvalue _returnvalue_2))
  (bind _returnvalue_4 (Math|Vector|Normalize _returnvalue_3 0.01))
  (bind _returnvalue_5 (* _returnvalue_4 1e+02))
  (bind _returnvalue_6 (+ _returnvalue_3 _returnvalue_5))
  (bind _returnvalue_7 (+ _returnvalue_6 ""))
  (Character|LaunchCharacter Affected (Math|Vector|MakeVector (.x _returnvalue_7) (.y _returnvalue_7) 1.5e+02) false false))

(fn BasicReactionSequence
  (params (Causer :type Actor%20Object%20Reference))
  (bind _returnvalue (Components|GetOwner))
  (bind _ascharacter (Utilities|Casting|CastToCharacter _returnvalue))
  (CallFunction|Hitstop _returnvalue false)
  (Reactions|Knockback _ascharacter Causer)
  (Reactions|Rotate Causer))

(fn Heal
  (params (Heal%20amount :type Float%20%28double-precision%29))
  (Variables|Default|SetHealth (Math|Float|Clamp(Float) (+ (Variables|Default|GetHealth) Heal%20amount) 0.0 (Variables|Default|GetMax%20Health)))
  (return))