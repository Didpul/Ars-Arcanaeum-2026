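; Actor component that tracks whether its owner is exposed to the level's Directional Light or obscured from it.
; On BeginPlay it caches the first Directional Light and starts a looping timer that runs a debug-drawn Visibility line trace from the owner.
; The trace end is the scaled owner-to-light-actor position vector, so it uses the light's location rather than its rotation.
; No hit sets HitByLight, a hit clears it, and LightValueChange is called only on changes.
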(event Custom|Trace
  (bind _returnvalue (Components|GetOwner))
  (bind _returnvalue_2 (Transformation|GetActorLocation _returnvalue))
  (bind _returnvalue_3 (Collision|LineTraceByChannel _returnvalue_2 (* (- (Transformation|GetActorLocation (Variables|Default|GetLight)) _returnvalue_2) 9999.0) "TraceTypeQuery1" false 0 "ForOneFrame"))
  (if (not _returnvalue_3)
    ;[1 1 1] lighten
    (if (not (Variables|Default|GetHit%20by%20light))
      (Variables|Default|SetHit%20by%20light true)
      (Default|CallLightValueChange))
    (else
      ;[1 1 1] obscured
      (if (Variables|Default|GetHit%20by%20light)
        (Variables|Default|SetHit%20by%20light false)
        (Default|CallLightValueChange)))))

(event EventTick
  (params (DeltaSeconds :type Float%20%28single-precision%29)))

(event EventBeginPlay
  (bind _returnvalue (Actor|GetActorOfClass "/Script/Engine.DirectionalLight"))
  (Variables|Default|SetLight _returnvalue)
  (Utilities|Time|SetTimerbyEvent (delegate Custom|Trace) 0.1 true))