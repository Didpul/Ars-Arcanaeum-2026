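; Soul orb pickup that drifts and bobs, homes in on an absorber and adds soul stability to it when absorbed.
; Tick combines periodically changing drift with noise-offset sine bobbing, eased by a timeline-driven value.
; LockAbsorber speeds it up toward the target; overlapping an absorbing actor triggers absorption, which notifies that actor and destroys the orb.
; If double spawning is allowed, BeginPlay has a random chance to spawn a health orb alongside it.
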(event OnComponentBeginOverlap(spherecol)
  (params (OverlappedComponent :type Primitive%20Component%20Object%20Reference) (OtherActor :type Actor%20Object%20Reference) (OtherComp :type Primitive%20Component%20Object%20Reference) (OtherBodyIndex :type Integer) (bFromSweep :type Boolean) (SweepResult :type Hit%20Result%20Structure%20%28by%20ref%29))
  (bind _absorbing_ (Class|BPISoulActor|CheckAbsorbing(Message) OtherActor))
  (if _absorbing_
    (Variables|Default|SetAbsorbing%20actor OtherActor)
    (Class|BPISoulActor|Absorption(Message) self)))

(event Custom|Change%20Dir
  (bind _returnvalue (Math|Random|RandomUnitVector))
  (Variables|Default|SetDriftDirection (Math|Interpolation|VInterpTo (Variables|Default|GetDriftDirection) (Math|Vector|MakeVector (.x _returnvalue) (.y _returnvalue) (.z (Math|Vector|SelectVector "0.000000,0.000000,1.000000" "0.000000,0.000000,-1.000000" (<= (.z (Variables|Default|GetDriftDirection)) 0.0)))) (stale EventTick DeltaSeconds) 1.0)))

(event EventBeginPlay
  (Utilities|FlowControl|Sequence
    (:then_0
      (Variables|Default|SetStart%20Location (Transformation|GetActorLocation))
      (Utilities|FlowControl|Sequence
        (:then_0
          (Variables|Default|SetNoise%20Offset (Math|Vector|MakeVector (Math|Random|RandomFloatinRange 0.0 1e+02) (Math|Random|RandomFloatinRange 0.0 1e+02) (Math|Random|RandomFloatinRange 0.0 1e+02)))
          (bind _returnvalue (Utilities|Time|SetTimerbyEvent (delegate Custom|Change%20Dir) 4.0 true))
          (Variables|Default|SetSwitch%20direction%20timer _returnvalue)
          (CallFunction|ChangeDir))
        (:then_1
          (Utilities|FlowControl|Delay 0.5)
          (bind _newtrack_0 (Timeline|Timeline PlayFromStart)
            (:Update
              (Variables|Default|Setswitch _newtrack_0))))))
    (:then_1
      (if (Variables|Default|GetCan%20double%20spawn)
        (switch int (Math|Random|RandomIntegerinRange 0 3)
          (:0
            (Game|SpawnActorfromClass "/Game/Characters/Soul_Orbs/BP_HealthOrb.BP_HealthOrb_C" (Transformation|GetActorTransform) "Undefined" "MultiplyWithRoot" 0 0 false 0)))))))

(event EventLockAbsorber
  (params (Absorber :type Actor%20Object%20Reference))
  (Variables|Default|Settarget%20actor Absorber)
  (Variables|Default|SetBeingAbsorbed true)
  (Variables|Default|SetDrift%20Speed 5e+02))

(event EventTick
  (params (DeltaSeconds :type Float%20%28single-precision%29))
  (bind _target_actor (Variables|Default|Gettarget%20actor))
  (Variables|Default|SetTimeAlive (+ (Variables|Default|GetTimeAlive) DeltaSeconds))
  (bind _output_get (Variables|Default|SetStart%20Location (+ (Variables|Default|GetStart%20Location) (* (* (Variables|Default|GetDriftDirection) (Variables|Default|GetDrift%20Speed)) DeltaSeconds))))
  (Transformation|SetActorLocation (Math|Interpolation|VInterpTo _output_get (+ (Variables|Default|GetStart%20Location) (Math|Vector|MakeVector (* (Math|Trig|Sin(Radians) (+ (* (Variables|Default|GetTimeAlive) 0.7) (.y (Variables|Default|GetNoise%20Offset)))) (Variables|Default|GetFloat%20Amplitude)) (* (Math|Trig|Cos(Radians) (+ (* (Variables|Default|GetTimeAlive) 0.9) (.z (Variables|Default|GetNoise%20Offset)))) (Variables|Default|GetFloat%20Amplitude)) (* (* (Math|Trig|Sin(Radians) (+ (* (Variables|Default|GetTimeAlive) (Variables|Default|GetFloat%20Speed)) (.x (Variables|Default|GetNoise%20Offset)))) (Variables|Default|GetFloat%20Amplitude)) 0.25))) (Variables|Default|Getswitch) 1.0) false false)
  (if (Variables|Default|GetBeingAbsorbed)
    (Utilities|IsValid _target_actor
      (:Is%20Valid
        (Variables|Default|SetDriftDirection (+ (Math|Vector|GetForwardVector (Math|Rotator|FindLookatRotation (Transformation|GetActorLocation) (Transformation|GetActorLocation _target_actor))) "0.000000,0.000000,0.100000")))
      (:Is%20Not%20Valid
        (Variables|Default|SetBeingAbsorbed false :!label _label)
        (Variables|Default|SetDrift%20Speed 3e+01)))
    (else
      (goto _label))))

(event EventAbsorption
  (bind _absorbing_actor (Variables|Default|GetAbsorbing%20actor))
  (Utilities|IsValid _absorbing_actor
    (:Is%20Valid
      (Class|BPISoulActor|ModifySoulStablity(Message) _absorbing_actor (Variables|Default|GetStabilityValue) true)
      (Class|BPISoulActor|Absorption(Message) _absorbing_actor)
      (Actor|DestroyActor))))

(event EventCancelAbsorb
  (Variables|Default|Settarget%20actor 0)
  (Variables|Default|SetBeingAbsorbed false))

(fn ConstructionScript)

(fn CheckAbsorbing
  (return false))

(fn ModifySoulStablity
  (params (Stability%20Amount :type Float%20%28double-precision%29) (Add :type Boolean))
  (return 0.0))