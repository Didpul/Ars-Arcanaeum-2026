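; Showcase character for Ars that runs a scripted movement and animation demo, starting on BeginPlay.
; It moves toward the orb spawner while a Timeline ramps walk speed, then plays a combo montage.
; A self-calling Play event then steps through a montage array, with Dash notifies launching the character forward, left, right or back by index.
; Combat interface functions are stubs apart from the combat component getter.
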(event Custom|play
  (bind _returnvalue (Transformation|GetActorForwardVector))
  (bind _returnvalue_2 (Transformation|GetActorRotation))
  (bind _returnvalue_3 (Math|Vector|GetRightVector _returnvalue_2))
  (bind _returnvalue_4 (Math|Vector|Normalize _returnvalue))
  (bind _returnvalue_5 (Math|Vector|Normalize _returnvalue_3))
  ;[1 1 1] Comment
  (bind _notifyname (Animation|Montage|PlayMontage (Variables|Character|GetMesh) (Utilities|Array|Get(acopy) (Variables|Default|GetMontage%20to%20Play) (Variables|Default|GetNewVar)) (Utilities|Operators|Divide 1.0 0.5 2.0))
    (:OnCompleted
      (Math|Integer|IncrementInt (Variables|Default|GetNewVar)
        (:%20%20
          (Utilities|FlowControl|Delay 0.2)
          (CallFunction|Play))))
    (:OnNotifyBegin
      (switch name _notifyname
        (:dash
          (Character|LaunchCharacter (Utilities|Select :Index (Variables|Default|GetNewVar) :Option%200 (* _returnvalue_4 3e+03) :Option%201 (* _returnvalue_5 -3e+03) :Option%202 (* _returnvalue_5 3e+03) :Option%203 (* _returnvalue_4 -3e+03)) true true))))))

(event Custom|combo%20show
  (Utilities|FlowControl|Delay 1.0)
  (Animation|Montage|PlayMontage (Variables|Character|GetMesh) "/Game/Ars_Combo1_montageSHOWCASE.Ars_Combo1_montageSHOWCASE" 1.0 0.0 "Stage1"
    (:OnCompleted
      (Utilities|FlowControl|Delay 1.0)
      (CallFunction|Play))
    (:OnBlendOut
      (Variables|Default|SetNewVar_0 true))))

(event EventBeginPlay
  (Variables|/Script/Engine.CharacterMovementComponent|SetMaxWalkSpeed (Variables|Character|GetCharacterMovement) 1e+02)
  (bind _returnvalue (Actor|GetActorOfClass "/Game/Characters/Soul_Orbs/BP_Orb_Spawner.BP_Orb_Spawner_C"))
  (AI|Navigation|SimpleMovetoLocation (Pawn|GetController) (Transformation|GetActorLocation _returnvalue))
  (Utilities|FlowControl|Delay 2.0)
  (bind _newtrack_0 (Timeline|Timeline Play)
    (:Update
      (Variables|/Script/Engine.CharacterMovementComponent|SetMaxWalkSpeed (Variables|Character|GetCharacterMovement) (Math|Float|Lerp 1e+02 5e+02 (Math|Float|NormalizetoRange _newtrack_0 0.0 1.0))))
    (:Finished
      (Utilities|FlowControl|Delay 1.0)
      (CallFunction|ComboShow))))

(fn ConstructionScript
  (Components|SkinnedMesh|SetLeaderPoseComponent (Variables|Default|Gethead) (Variables|Character|GetMesh) false false))

(fn GetActiveTarget
  (return 0))

(fn GetTeamNumber
  (return 0))

(fn GetCombatComp
  (return (Variables|Default|GetBpC_Combat)))

(fn Heal
  (params (Heal%20Amount :type Float%20%28double-precision%29))
  (return false))

(fn ReceiveDamage
  (params (Damage%20Causer :type Actor%20Object%20Reference) (Damage%20Info :type S%20Damage%20Info%20Structure))
  (return false))

(fn Stun
  (return false))