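; BP_HealthOrb is a soul orb variant that heals the actor absorbing it.
; On BeginPlay it runs the parent logic, then tints its Niagara system green.
; Its Absorption event checks that AbsorbingActor is valid, sends it a heal message using StabilityValue and an absorption message, then destroys the orb.
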(event EventBeginPlay
  (|CallParentFunction)
  (Niagara|SetNiagaraVariable(LinearColor) (Variables|Default|GetNewNiagaraSystem) "Color" (Math|Color|MakeColor 0.0 1.0 0.0)))

(event Collision|EventActorBeginOverlap
  (params (OtherActor :type Actor%20Object%20Reference)))

(event EventTick
  (params (DeltaSeconds :type Float%20%28single-precision%29))
  (|CallParentFunction DeltaSeconds) ; This node is disabled and will not be called.\nDrag off pins to build functionality.
)

(event EventAbsorption
  (bind _absorbing_actor (Variables|Default|GetAbsorbing%20actor))
  (Utilities|IsValid _absorbing_actor
    (:Is%20Valid
      (Class|BPIDamageable|Heal(Message) _absorbing_actor (Variables|Default|GetStabilityValue))
      (Class|BPISoulActor|Absorption(Message) _absorbing_actor)
      (Actor|DestroyActor))))

(fn ConstructionScript
  (|CallParentFunction))