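; BP_Base_Enemy is the base enemy character, delegating damage, death state and team number to its BpCCombat component.
; It registers with BP_Combat_Manager on BeginPlay, then on death unregisters, returns any held attack token and destroys itself.
; Lock-on toggles a Niagara aim circle at FocusPoint, and ChangeSpeed maps AI state to walk speed.
; Getters expose components and data, with several left as stubs, as are Heal and Stun.
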(event Custom|Death
  (bind _self self)
  (bind _combat_manager (Variables|Default|GetCombat%20Manager))
  (Variables|/Game/Components/BpC_Combat.BpC_Combat_C|SetDead (Variables|Default|GetBpC_Combat) true)
  (Default|UnRegisterActor (Variables|Default|GetCombat%20Manager) self)
  (if (Utilities|Array|ContainsItem (Variables|/Game/Core/CombatManager/BP_Combat_Manager.BP_Combat_Manager_C|GetAttacker%20List _combat_manager) _self)
    (Default|ReturnToken _combat_manager _self))
  (Actor|DestroyActor))

(event EventBeginPlay
  (bind _returnvalue (Actor|GetActorOfClass "/Game/Core/CombatManager/BP_Combat_Manager.BP_Combat_Manager_C"))
  (Utilities|IsValid _returnvalue
    (:Is%20Valid
      (bind _output_get (Variables|Default|SetCombat%20Manager _returnvalue))
      (Default|RegisterActor _output_get self))))

(event EventLockedasTarget
  (params (On/Off :type Boolean))
  (bind _focus_point (Variables|Default|GetFocus%20Point))
  (if On/Off
    (bind _returnvalue (Niagara|SpawnSystemAttached "/Game/Art/NFX/NFX_Circle_Aim.NFX_Circle_Aim" _focus_point (Transformation|GetAttachSocketName _focus_point) (Transformation|GetWorldLocation (Variables|Default|GetFocus%20Point)) "0, 0, 0" "KeepWorldPosition" false))
    (Variables|Default|SetLocked%20FX _returnvalue)
    (Effects|Components|ParticleSystem|SetFloatParameter _returnvalue "User.Size" 2.0)
    (Development|PrintString "Hello")
    (else
      (bind _locked_fx (Variables|Default|GetLocked%20FX)
        (:then
          (Components|DestroyComponent _locked_fx))
        (:else)))))

(fn ConstructionScript
  (bind _mesh (Variables|Character|GetMesh))
  (|CallParentFunction)
  (bind _returnvalue (Rendering|Material|CreateDynamicMaterialInstance _mesh 0 (Rendering|Material|GetMaterial _mesh 0) "None" :!class /Script/Engine.PrimitiveComponent))
  (Variables|Default|SetBase_Mat _returnvalue))

(fn ChangeSpeed
  (params (State :type E_Enemy_States%20Enum :default "NewEnumerator0"))
  (bind _output_get (Variables|/Script/Engine.CharacterMovementComponent|SetMaxWalkSpeed (Variables|Character|GetCharacterMovement) (Utilities|Select :Index State :NewEnumerator0 1e+02 :NewEnumerator1 3e+02 :NewEnumerator5 1.5e+02 :NewEnumerator2 0.0 :NewEnumerator3 0.0 :NewEnumerator4 0.0)))
  (return _output_get))

(fn CombatManagerInteraction
  (return (Variables|Default|GetCombat%20Manager)))

(fn DeadCheck
  (return (Variables|/Game/Components/BpC_Combat.BpC_Combat_C|GetDead (Variables|Default|GetBpC_Combat))))

(fn GetSoulComp
  (return 0))

(fn GetActiveTarget
  (return 0))

(fn GetCameraComponent
  (return 0 0))

(fn GetCapsulle
  (return 0))

(fn GetDataAsset
  (return (Variables|Default|GetData%20Asset)))

(fn GetMaterial
  (return 0 false 0))

(fn GetMovementComp
  (return (Variables|Character|GetCharacterMovement)))

(fn GetTarget
  (return 0))

(fn GetTeamNumber
  (return (Variables|/Game/Components/BpC_Combat.BpC_Combat_C|GetTeam%20number (Variables|Default|GetBpC_Combat))))

(fn GetCombatComp
  (return (Variables|Default|GetBpC_Combat)))

(fn GetMesh
  (return (Variables|Character|GetMesh)))

(fn Heal
  (params (Heal%20Amount :type Float%20%28double-precision%29))
  (return false))

(fn ReceiveDamage
  (params (Damage%20Causer :type Actor%20Object%20Reference) (Damage%20Info :type S%20Damage%20Info%20Structure))
  (bind _should_react (Default|DamageReceived (Variables|Default|GetBpC_Combat) Damage%20Causer Damage%20Info))
  (return _should_react))

(fn Stun
  (return false))