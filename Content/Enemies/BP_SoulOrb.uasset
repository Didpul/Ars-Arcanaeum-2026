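; Soul orb that drifts and bobs in the air until an absorber takes it in.
; Tick moves a base location along a periodically randomized direction, layering per-instance sine/cosine wobble on top.
; A seek timer sphere-traces for nearby Pawns; a hit or Absorb call makes the orb speed toward that target.
; Overlapping an actor that confirms it is absorbing sends AbsorptionMessage and destroys the orb.
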(event OnComponentBeginOverlap(spherecol)
  (params (OverlappedComponent :type Primitive%20Component%20Object%20Reference) (OtherActor :type Actor%20Object%20Reference) (OtherComp :type Primitive%20Component%20Object%20Reference) (OtherBodyIndex :type Integer) (bFromSweep :type Boolean) (SweepResult :type Hit%20Result%20Structure%20%28by%20ref%29))
  (bind _absorbing_ (Class|BPISoulActor|CheckAbsorbing(Message) OtherActor))
  (if _absorbing_
    (Class|BPISoulActor|Absorption(Message) OtherActor)
    (Actor|DestroyActor)))

(event Custom|Change%20Dir
  (bind _returnvalue (Math|Random|RandomUnitVector))
  (Variables|Default|SetDriftDirection (Math|Interpolation|VInterpTo (Variables|Default|GetDriftDirection) (Math|Vector|MakeVector (.x _returnvalue) (.y _returnvalue) (.z (Math|Vector|SelectVector "0.000000,0.000000,1.000000" "0.000000,0.000000,-1.000000" (<= (.z (Variables|Default|GetDriftDirection)) 0.0)))) (stale EventTick DeltaSeconds) 1.0)))

(event Custom|go%20to
  (bind _returnvalue (Transformation|GetActorLocation))
  (bind (_outhit _returnvalue_2) (Collision|SphereTraceForObjects _returnvalue _returnvalue 1.5e+03 (Utilities|Array|MakeArray "ObjectTypeQuery3") false 0 "ForOneFrame"))
  (if _returnvalue_2
    (Variables|Default|Settarget%20actor (.HitActor (Collision|BreakHitResult _outhit)))
    (Variables|Default|SetBeingAbsorbed true)
    (Utilities|Time|ClearandInvalidateTimerbyHandle (Variables|Default|GetSwitch%20direction%20timer))
    (Variables|Default|SetDrift%20Speed 5e+02)
    (else
      (CallFunction|ResetTimer))))

(event Custom|reset%20timer
  (bind _returnvalue (Utilities|Time|SetTimerbyEvent (delegate Custom|go%20to) 1e+01))
  (Variables|Default|SetSeek%20timer _returnvalue))

(event EventBeginPlay
  (Variables|Default|SetStart%20Location (Transformation|GetActorLocation))
  (Utilities|FlowControl|Sequence
    (:then_0
      (Variables|Default|SetNoise%20Offset (Math|Vector|MakeVector (Math|Random|RandomFloatinRange 0.0 1e+02) (Math|Random|RandomFloatinRange 0.0 1e+02) (Math|Random|RandomFloatinRange 0.0 1e+02)))
      (bind _returnvalue (Utilities|Time|SetTimerbyEvent (delegate Custom|Change%20Dir) 4.0 true))
      (Variables|Default|SetSwitch%20direction%20timer _returnvalue)
      (CallFunction|ChangeDir)
      (bind _returnvalue_2 (Utilities|Time|SetTimerbyEvent (delegate Custom|go%20to) 1e+01))
      (Variables|Default|SetSeek%20timer _returnvalue_2))
    (:then_1
      (Utilities|FlowControl|Delay 0.5)
      (bind _newtrack_0 (Timeline|Timeline PlayFromStart)
        (:Update
          (Variables|Default|Setswitch _newtrack_0))))))

(event EventTick
  (params (DeltaSeconds :type Float%20%28single-precision%29))
  (bind _target_actor (Variables|Default|Gettarget%20actor))
  (Variables|Default|SetTimeAlive (+ (Variables|Default|GetTimeAlive) DeltaSeconds))
  (bind _output_get (Variables|Default|SetStart%20Location (+ (Variables|Default|GetStart%20Location) (* (* (Variables|Default|GetDriftDirection) (Variables|Default|GetDrift%20Speed)) DeltaSeconds))))
  (Transformation|SetActorLocation (Math|Interpolation|VInterpTo _output_get (+ (Variables|Default|GetStart%20Location) (Math|Vector|MakeVector (* (Math|Trig|Sin(Radians) (+ (* (Variables|Default|GetTimeAlive) 0.7) (.y (Variables|Default|GetNoise%20Offset)))) (Variables|Default|GetFloat%20Amplitude)) (* (Math|Trig|Cos(Radians) (+ (* (Variables|Default|GetTimeAlive) 0.9) (.z (Variables|Default|GetNoise%20Offset)))) (Variables|Default|GetFloat%20Amplitude)) (* (* (Math|Trig|Sin(Radians) (+ (* (Variables|Default|GetTimeAlive) (Variables|Default|GetFloat%20Speed)) (.x (Variables|Default|GetNoise%20Offset)))) (Variables|Default|GetFloat%20Amplitude)) 0.25))) (Variables|Default|Getswitch) 1.0) false false)
  (if (Variables|Default|GetBeingAbsorbed)
    (Utilities|IsValid _target_actor
      (:Is%20Valid
        (Variables|Default|SetDriftDirection (+ (Math|Vector|GetForwardVector (Math|Rotator|FindLookatRotation (Transformation|GetActorLocation) (Transformation|GetActorLocation _target_actor))) "0.000000,0.000000,0.100000")))
      (:Is%20Not%20Valid
        (Variables|Default|SetBeingAbsorbed false)
        (CallFunction|ResetTimer)
        (Variables|Default|SetDrift%20Speed 3e+01)))))

(event EventAbsorb
  (params (Absorber :type Actor%20Object%20Reference))
  (bind _seek_timer (Variables|Default|GetSeek%20timer))
  (Variables|Default|Settarget%20actor Absorber)
  (if (Utilities|Time|IsValidTimerHandle _seek_timer)
    (Utilities|Time|ClearandInvalidateTimerbyHandle _seek_timer))
  (Variables|Default|SetBeingAbsorbed true)
  (Utilities|Time|ClearandInvalidateTimerbyHandle (Variables|Default|GetSwitch%20direction%20timer))
  (Variables|Default|SetDrift%20Speed 5e+02))

(event EventCancelAbsorb
  (Variables|Default|Settarget%20actor 0)
  (Variables|Default|SetBeingAbsorbed false)
  (CallFunction|ResetTimer))

(fn ConstructionScript)

(fn CheckAbsorbing
  (return false))