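; BP_Combat_Manager coordinates combat actors by limiting simultaneous attackers with a shared token pool.
; Actors register in ActorList, while RequestAttack and RequestState grant tokens up to MaxTokens and track holders in AttackerList.
; ReturnToken frees a slot, and RequestState picks one of two fallback states at random when the pool is full.
; CheckAttackDistance selects a state by comparing target distance to the actor's data-asset passive and attack radii.
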(event Custom|ForceReturn
  (CallFunction|ReturnToken))

(event EventBeginPlay)

(event EventTick
  (params (DeltaSeconds :type Float%20%28single-precision%29)))

(fn ConstructionScript)

(fn RegisterActor
  (params (ACtor :type Actor%20Object%20Reference%20%28by%20ref%29))
  (Utilities|Array|AddUnique (Variables|Default|GetActor%20List) ACtor)
  (Development|PrintString (Utilities|String|Append "Added Actor" (Utilities|GetDisplayName ACtor))))

(fn UnRegisterActor
  (params (ACtor :type Actor%20Object%20Reference%20%28by%20ref%29))
  (Utilities|Array|RemoveItem (Variables|Default|GetActor%20List) ACtor)
  (Development|PrintString (Utilities|String|Append "Removed Actor" (Utilities|GetDisplayName ACtor))))

(fn RequestAttack
  (params (Requester :type Actor%20Object%20Reference))
  (if (<= (Variables|Default|GetActive%20Tokens) (Variables|Default|GetMax%20Tokens))
    (if (> (+ (Variables|Default|GetActive%20Tokens) 1) (Variables|Default|GetMax%20Tokens))
      _
      (else
        (Variables|Default|SetActive%20Tokens (+ (Variables|Default|GetActive%20Tokens) 1))
        (Utilities|Array|Add (Variables|Default|GetAttacker%20List) Requester)
        (return true))))
  (return false))

(fn ReturnToken
  (params (Attacker%20 :type Actor%20Object%20Reference))
  (Variables|Default|SetActive%20Tokens (Math|Integer|Clamp(Integer) (- (Variables|Default|GetActive%20Tokens) 1) 0 (Variables|Default|GetMax%20Tokens)))
  (Utilities|Array|RemoveItem (Variables|Default|GetAttacker%20List) Attacker%20))

(fn RequestState
  (params (Actor%20asking%20permission :type Actor%20Object%20Reference%20%28by%20ref%29))
  (bind _attacker_list (Variables|Default|GetAttacker%20List))
  (if (< (Variables|Default|GetActive%20Tokens) (Variables|Default|GetMax%20Tokens))
    (if (Utilities|Array|ContainsItem _attacker_list Actor%20asking%20permission)
      (Utilities|Array|RemoveItem (Variables|Default|GetAttacker%20List) Actor%20asking%20permission)
      (return "NewEnumerator3")
      (else
        (Math|Integer|IncrementInt (Variables|Default|GetActive%20Tokens)
          (:%20%20
            (Utilities|Array|AddUnique _attacker_list Actor%20asking%20permission)
            (return "NewEnumerator0")))))
    (else
      (return (Utilities|Select :Index (Math|Random|RandomIntegerinRange 0 1) :Option%200 "NewEnumerator2" :Option%201 "NewEnumerator1")))))

(fn RemovefromArray
  (params (Item :type Actor%20Object%20Reference%20%28by%20ref%29))
  (bind _attacker_list (Variables|Default|GetAttacker%20List))
  (if (Utilities|Array|ContainsItem _attacker_list Item)
    (Utilities|Array|RemoveItem _attacker_list Item)))

(fn CheckAttackDistance
  (params (Actor :type Actor%20Object%20Reference))
  (bind _data_asset (Class|BPIEnemyActions|GetDataAsset(Message) Actor))
  (bind _target_actor (Class|BPIEnemyActions|GetTarget(Message) Actor))
  (if (> (Math|Vector|Distance(Vector) (Transformation|GetActorLocation Actor) (Transformation|GetActorLocation _target_actor)) (Variables|/Game/Enemies/Data_Assets/DA_EnemyBase.DA_EnemyBase_C|GetPassive%20Radius _data_asset))
    (return "NewEnumerator6")
    (elif (< (Math|Vector|Distance(Vector) (Transformation|GetActorLocation Actor) (Transformation|GetActorLocation _target_actor)) (Variables|/Game/Enemies/Data_Assets/DA_EnemyBase.DA_EnemyBase_C|GetAttack%20Radius _data_asset))
      (return "NewEnumerator1")
      (else
        (return "NewEnumerator5")))))