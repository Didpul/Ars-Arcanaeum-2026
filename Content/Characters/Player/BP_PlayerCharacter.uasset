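; Player character for action combat with combo melee, typed spell casting, lock-on and soul absorption, gated by a CurrentState enum.
; Combat, Soul and Spells components handle health, stability and casting; absorbed souls heal or restore stability, and soul state scales damage taken.
; Lock-on turns jump into a directional timeline dash, frames the target midpoint and zooms by distance, with a timer breaking it at range.
; Includes debug slow-motion and stat printouts.
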(event Custom|Start%20attacking
  ;[1 0.5318 0.452 1 40] Attack
  (Variables|Default|SetCurrentState "NewEnumerator2")
  (Animation|Montage|PlayMontage (Variables|Character|GetMesh) "/Game/Characters/Player/Montages/Ars_Combo1_montage.Ars_Combo1_montage" 1.0 0.0 (Variables|Default|GetComboStage)))

(event Custom|Dash
  ;[0.6403 1 0.4605 1 40] Dash
  (if (Utilities|Enum|NotEqual(Enum) (Variables|Default|GetCurrentState) "NewEnumerator7")
    (Variables|Default|SetCurrentState "NewEnumerator7")
    (CallFunction|CheckDashDirection)
    (Animation|Montage|PlayMontage (Variables|Character|GetMesh) (Utilities|Select :Index (Variables|Default|GetDashDirection) :Option%200 "/Game/Characters/Player/Animations/Dashes/Dash_F_NwO_Montage.Dash_F_NwO_Montage" :Option%201 "/Game/Characters/Player/Animations/Dashes/DASH_B_Montage.DASH_B_Montage" :Option%202 "/Game/Characters/Player/Animations/Dashes/DASH_L_Montage.DASH_L_Montage" :Option%203 "/Game/Characters/Player/Animations/Dashes/DASH_R_Montage.DASH_R_Montage") (Utilities|Operators|Divide 0.8 0.2 2.0)
      (:then
        (CallFunction|MoveDash (CallFunction|DashDistance)))
      (:OnCompleted
        (Variables|Default|SetDashDirection 1)
        (Variables|Default|SetCurrentState "NewEnumerator0")))))

(event Custom|release%20area
  ;[0.349 0 0 1 74] Experimental
  (bind _notifyname (Animation|Montage|PlayMontage (Variables|Character|GetMesh) "/Game/Characters/Player/Animations/NWO26_QuickSpell1_Montage.NWO26_QuickSpell1_Montage")
    (:OnCompleted
      (Variables|Default|SetCurrentState "NewEnumerator0" :!label _label))
    (:OnInterrupted
      (goto _label))
    (:OnNotifyBegin
      (switch name _notifyname
        (:cast
          (Default|CastSpell (Variables|Default|GetBPC_Spells) (Variables|Default|GetActive%20Spell)))))))

(event Custom|MoveDash
  (params (Location :type Vector))
  (bind _returnvalue (Transformation|GetActorLocation))
  (bind (_x _y) (Math|Vector|BreakVector Location))
  ;[0.6403 1 0.4605 1 40] Dash
  (bind _dashtrack (Timeline|DashTimeline PlayFromStart)
    (:Update
      (Transformation|SetActorLocation (Math|Vector|Lerp(Vector) _returnvalue (Math|Vector|MakeVector _x _y (.Z (Math|Vector|BreakVector _returnvalue))) _dashtrack) true true))))

(event Custom|Check%20distance%20to%20target
  (bind _locked_actor (Variables|Lock|GetLocked%20actor))
  (bind _springarm (Variables|Default|GetSpringArm))
  ;[1 0.5318 0.452 1 40] Lock Tick behaviour
  (Utilities|IsValid _locked_actor
    (:Is%20Valid
      (Variables|/Script/Engine.SpringArmComponent|SetTargetArmLength _springarm (Math|Interpolation|FInterpTo (Variables|/Script/Engine.SpringArmComponent|GetTargetArmLength _springarm) (Math|Float|MapRangeClamped (Math|Vector|Distance(Vector) (Transformation|GetActorLocation _locked_actor) (Transformation|GetActorLocation)) (Variables|Lock|GetMin%20Distance) (Variables|Lock|GetMax%20Distance) (Variables|Lock|GetMin%20Zoom) (Variables|Lock|GetMax%20Zoom)) (Utilities|Time|GetWorldDeltaSeconds) 1e+01)))))

(event Custom|unfreeze
  (bind _charactermovement (Variables|Character|GetCharacterMovement))
  ;[0.2488 0.9602 1 1 40] Freeze/unfreeze
  (Variables|/Script/Engine.CharacterMovementComponent|SetMaxWalkSpeed _charactermovement (Math|Float|SelectFloat 2.5e+02 5e+02 (Variables|Lock|GetLocked%20)))
  (Variables|/Script/Engine.CharacterMovementComponent|SetRotationRate _charactermovement "0.000000,1080.000000,0.000000")
  (Variables|Default|SetCurrentState "NewEnumerator0"))

(event Custom|freeze
  (bind _charactermovement (Variables|Character|GetCharacterMovement))
  ;[0.2488 0.9602 1 1 40] Freeze/unfreeze
  (Variables|/Script/Engine.CharacterMovementComponent|SetMaxWalkSpeed _charactermovement 0.0)
  (Variables|/Script/Engine.CharacterMovementComponent|SetRotationRate _charactermovement "0, 0, 0"))

(event Custom|resettt
  ;[1 0.5318 0.452 1 40] Lock Tick behaviour
  (bind _newtrack_0 (Timeline|reset%20cam PlayFromStart)
    (:Update
      (Transformation|SetWorldRotation (Variables|Default|GetCamera) (Math|Interpolation|RInterpTo (Transformation|GetWorldRotation (Variables|Default|GetCamera)) (Variables|Lock|GetCamera%20Previous%20rotation) _newtrack_0 5.0) false false))))

(event Custom|On%20Melee%20Hit
  ;[1 0.5318 0.452 1 40] Attack
  (Default|ModifyStability (Variables|Default|GetBPC_Soul) 1e+01 true))

(event Custom|Start%20Absorb
  (bind _returnvalue (Transformation|GetActorLocation))
  ;[0.8184 0.3355 1 1 40] Soul Absorption
  (switch Utilities|FlowControl|Switch|SwitchonE_CombatStates (Variables|Default|GetCurrentState)
    (:NewEnumerator0
      _)
    (:NewEnumerator5
      _)
    (:NewEnumerator8
      _))
  (Variables|Default|SetCurrentState "NewEnumerator8")
  (CallFunction|Freeze)
  (bind _outhits (Collision|MultiSphereTraceForObjects _returnvalue _returnvalue 1.5e+03 (Utilities|Array|MakeArray "ObjectTypeQuery2") false 0 "ForDuration"))
  (for _array_element _outhits
    (if (Utilities|DoesObjectImplementInterface (.HitActor (Collision|BreakHitResult _array_element)) "/Game/Interfaces/BPI_SoulActor.BPI_SoulActor_C")
      (Utilities|Array|AddUnique (Variables|Default|GetSouls%20Absorbing) (.HitActor (Collision|BreakHitResult _array_element)))
      (Class|BPISoulActor|Absorb(Message) (.HitActor (Collision|BreakHitResult _array_element)) self))))

(event Custom|Stop%20Absorb
  ;[0.8184 0.3355 1 1 40] Soul Absorption
  (Variables|Default|SetCurrentState "NewEnumerator0")
  (CallFunction|Unfreeze)
  (for _array_element (Variables|Default|GetSouls%20Absorbing)
    (Utilities|IsValid _array_element
      (:Is%20Valid
        (Class|BPISoulActor|CancelAbsorb(Message) _array_element)))))

(event Input|EnhancedActionEvents|EnhancedInputActionIA_Move
  (params (ActionValue :type Vector%202D%20Structure) (ElapsedSeconds :type Float%20%28double-precision%29) (TriggeredSeconds :type Float%20%28double-precision%29) (InputAction :type Input%20Action%20Object%20Reference :default "/Game/Core/Input/IA_Move.IA_Move"))
  (bind _returnvalue (Pawn|GetControlRotation :!class /Script/Engine.Pawn))
  ;[0.4181 1 0.5565 1 40] Movement
  (Pawn|Input|AddMovementInput (Math|Vector|GetRightVector (Math|Rotator|MakeRotator (.roll _returnvalue) 0.0 (.yaw _returnvalue))) (.x ActionValue) false)
  (Pawn|Input|AddMovementInput (Math|Vector|GetForwardVector (Math|Rotator|MakeRotator 0.0 0.0 (.yaw _returnvalue))) (.y ActionValue) false))

(event Input|EnhancedActionEvents|EnhancedInputActionIA_Look
  (params (ActionValue :type Vector%202D%20Structure) (ElapsedSeconds :type Float%20%28double-precision%29) (TriggeredSeconds :type Float%20%28double-precision%29) (InputAction :type Input%20Action%20Object%20Reference :default "/Game/Core/Input/IA_Look.IA_Look"))
  ;[0.4181 1 0.5565 1 40] Movement
  (if (not (Variables|Lock|GetLocked%20))
    (Pawn|Input|AddControllerYawInput (.x ActionValue))
    (Pawn|Input|AddControllerPitchInput (* (.y ActionValue) -1.0))))

(event Input|EnhancedActionEvents|EnhancedInputActionIA_Attack
  (params (ActionValue :type Boolean) (ElapsedSeconds :type Float%20%28double-precision%29) (TriggeredSeconds :type Float%20%28double-precision%29) (InputAction :type Input%20Action%20Object%20Reference :default "/Game/Core/Input/IA_Attack.IA_Attack"))
  ;[1 0.5318 0.452 1 40] Attack
  (switch Utilities|FlowControl|Switch|SwitchonE_CombatStates (Variables|Default|GetCurrentState)
    (:NewEnumerator0
      _)
    (:NewEnumerator5
      _))
  (CallFunction|StartAttacking)
  (Default|SoftLock (Variables|Default|GetBpC_Combat)))

(event Input|EnhancedActionEvents|EnhancedInputActionIA_Jump
  (params (ActionValue :type Boolean) (ElapsedSeconds :type Float%20%28double-precision%29) (TriggeredSeconds :type Float%20%28double-precision%29) (InputAction :type Input%20Action%20Object%20Reference :default "/Game/Core/Input/IA_Jump.IA_Jump"))
  ;[0.4181 1 0.5565 1 40] Movement
  (if (not (Variables|Lock|GetLocked%20))
    (switch Utilities|FlowControl|Switch|SwitchonE_CombatStates (Variables|Default|GetCurrentState)
      (:NewEnumerator0
        _)
      (:NewEnumerator5
        _))
    (Character|Jump)
    (Variables|Default|SetCurrentState "NewEnumerator6")
    (else
      (CallFunction|Dash))))

(event Input|EnhancedActionEvents|EnhancedInputActionIA_Lock
  (params (ActionValue :type Boolean) (ElapsedSeconds :type Float%20%28double-precision%29) (TriggeredSeconds :type Float%20%28double-precision%29) (InputAction :type Input%20Action%20Object%20Reference :default "/Game/Core/Input/IA_Lock.IA_Lock"))
  ;[1 0.5318 0.452 1 40] Lock on/off
  (if (Utilities|Enum|NotEqual(Enum) (Variables|Default|GetCurrentState) "NewEnumerator8")
    (if (Variables|Lock|GetLocked%20)
      (CallFunction|DisengageLock)
      (else
        (CallFunction|EngageLock)))))

(event Input|EnhancedActionEvents|EnhancedInputActionIA_Absorb
  (params (ActionValue :type Boolean) (ElapsedSeconds :type Float%20%28double-precision%29) (TriggeredSeconds :type Float%20%28double-precision%29) (InputAction :type Input%20Action%20Object%20Reference :default "/Game/Core/Input/IA_Absorb.IA_Absorb"))
  ;[0.8184 0.3355 1 1 40] Soul Absorption
  ;;[0 0.9206 1] Input
  (:Triggered
    (if (not (Variables|Lock|GetLocked%20))
      (CallFunction|StartAbsorb)))
  (:Canceled
    (CallFunction|StopAbsorb)))

(event Input|EnhancedActionEvents|EnhancedInputActionIA_Cast
  (params (ActionValue :type Boolean) (ElapsedSeconds :type Float%20%28double-precision%29) (TriggeredSeconds :type Float%20%28double-precision%29) (InputAction :type Input%20Action%20Object%20Reference :default "/Game/Core/Input/IA_Cast.IA_Cast"))
  ;[0.349 0 0 1 74] Experimental
  (:Started
    (switch Utilities|FlowControl|Switch|SwitchonE_SpellTypes (Variables|/Game/Spells/PDA_Spells.PDA_Spells_C|GetSpell%20Type (Variables|Default|GetActive%20Spell))
      (:NewEnumerator0
        _)
      (:NewEnumerator3
        _)
      (:NewEnumerator4
        _)
      (:NewEnumerator5
        _))
    (switch Utilities|FlowControl|Switch|SwitchonE_CombatStates (Variables|Default|GetCurrentState)
      (:NewEnumerator0
        _)
      (:NewEnumerator5
        _))
    (Variables|Default|SetCurrentState "NewEnumerator9")
    (CallFunction|SetActiveSpell)
    (bind _notifyname (Animation|Montage|PlayMontage (Variables|Character|GetMesh) "/Game/Characters/Player/Animations/NWO26_QuickSpell1_Montage.NWO26_QuickSpell1_Montage")
      (:OnCompleted
        (Variables|Default|SetCurrentState "NewEnumerator0" :!label _label))
      (:OnInterrupted
        (goto _label))
      (:OnNotifyBegin
        (switch name _notifyname
          (:cast
            (Default|CastSpell (Variables|Default|GetBPC_Spells) (Variables|Default|GetActive%20Spell)))))))
  (:Completed
    (Default|CancelCast (Variables|Default|GetBPC_Spells))
    (switch Utilities|FlowControl|Switch|SwitchonE_SpellTypes (Variables|/Game/Spells/PDA_Spells.PDA_Spells_C|GetSpell%20Type (Variables|Default|GetActive%20Spell))
      (:NewEnumerator5
        (Animation|StopAnimMontage (Animation|GetCurrentMontage :!class /Script/Engine.Character))))))

(event Input|EnhancedActionEvents|EnhancedInputActionIA_Release
  (params (ActionValue :type Boolean) (ElapsedSeconds :type Float%20%28double-precision%29) (TriggeredSeconds :type Float%20%28double-precision%29) (InputAction :type Input%20Action%20Object%20Reference :default "/Game/Core/Input/IA_Release.IA_Release"))
  (bind _active_spell (Variables|Default|GetActive%20Spell))
  (bind _bpc_spells (Variables|Default|GetBPC_Spells))
  (bind _spell_type (Variables|/Game/Spells/PDA_Spells.PDA_Spells_C|GetSpell%20Type _active_spell))
  (bind _returnvalue (Utilities|Enum|Equal(Enum) _spell_type "NewEnumerator1"))
  ;[0.349 0 0 1 74] Experimental
  (:Triggered
    (if _returnvalue
      (Utilities|FlowControl|DoOnce false :!label _label
        (:Completed
          (switch Utilities|FlowControl|Switch|SwitchonE_CombatStates (Variables|Default|GetCurrentState)
            (:NewEnumerator0
              _)
            (:NewEnumerator5
              _)
            (:NewEnumerator9
              _))
          (Variables|Default|SetCurrentState "NewEnumerator9")
          (CallFunction|SetActiveSpell)
          (Default|StartAreaTrace (Variables|Default|GetBPC_Spells))))))
  (:Completed
    (if _returnvalue
      (if (Utilities|Operators|NotEqual(!=) :A (Variables|/Game/Components/BPC_Spells.BPC_Spells_C|GetArea%20Location _bpc_spells))
        (CallFunction|ReleaseArea)
        (goto _label Reset)
        (else
          (Default|CancelAreaTrace _bpc_spells)
          (Variables|Default|SetCurrentState "NewEnumerator0")
          (goto _label Reset))))))

(event EventOnLanded
  (params (Hit :type Hit%20Result%20Structure%20%28by%20ref%29))
  ;[0.4181 1 0.5565 1 40] Movement
  (Variables|Default|SetCurrentState "NewEnumerator0"))

(event EventTick
  (params (DeltaSeconds :type Float%20%28single-precision%29))
  (bind _returnvalue (Transformation|GetActorRotation))
  (bind _camera (Variables|Default|GetCamera))
  ;[1 0.5318 0.452 1 40] Lock Tick behaviour
  (Utilities|FlowControl|Sequence
    (:then_0
      (if (Variables|Lock|GetLocked%20)
        (Utilities|IsValid (Variables|Lock|GetLocked%20actor)
          (:Is%20Valid
            (Transformation|SetActorRotation (Math|Rotator|MakeRotator (.roll _returnvalue) (.pitch _returnvalue) (.yaw (Math|Rotator|FindLookatRotation (Transformation|GetActorLocation) (Transformation|GetActorLocation (Variables|Lock|GetLocked%20actor))))))
            (Transformation|SetWorldRotation (Variables|Default|GetCamera) (Math|Interpolation|RInterpTo (Transformation|GetWorldRotation _camera) (Math|Rotator|FindLookatRotation (Transformation|GetWorldLocation _camera) (* (+ (Transformation|GetActorLocation (Variables|Lock|GetLocked%20actor)) (Transformation|GetActorLocation)) 0.5)) DeltaSeconds 5.0) false false)
            (CallFunction|CheckDistancetoTarget))
          (:Is%20Not%20Valid
            (CallFunction|DisengageLock)))))
    (:then_1
      (Development|PrintString (Utilities|String|ToString(Float) (Variables|/Game/Components/BpC_Combat.BpC_Combat_C|GetHealth (Variables|Default|GetBpC_Combat))) true true "(R=0.000000,G=1.000000,B=0.951951,A=1.000000)" DeltaSeconds)
      (Development|PrintString (Utilities|String|ToString(Float) (Variables|/Game/Components/BPC_Soul.BPC_Soul_C|GetSoulStability (Variables|Default|GetBPC_Soul))) true true "(R=1.000000,G=0.826772,B=0.000000,A=1.000000)" DeltaSeconds))))

(event EventDie
  (params (Spell? :type Boolean) (Killer :type Actor%20Object%20Reference))
  ;[1 0.5318 0.452 1 50] Receive Damage
  (Game|OpenLevel(byObjectReference) "/Game/Untitled.Untitled"))

(event EventDamageReaction
  (params (Damage%20Causer :type Actor%20Object%20Reference) (Damage%20Type :type E_DamageTypes%20Enum :default "NewEnumerator6"))
  ;[1 0.5318 0.452 1 50] Receive Damage
  (if (or (Utilities|Enum|Equal(Enum) (Variables|Default|GetCurrentState) "NewEnumerator8") (Utilities|Enum|Equal(Enum) (Variables|Default|GetCurrentState) "NewEnumerator9"))
    (Default|ModifyStability (Variables|Default|GetBPC_Soul) 2e+01 false))
  (CallFunction|StopAbsorb)
  (Variables|Default|SetCurrentState "NewEnumerator3")
  (CallFunction|Freeze)
  (Animation|Montage|PlayMontage (Variables|Character|GetMesh) "/Game/Characters/Player/Animations/Damaged_Combat_Montage.Damaged_Combat_Montage"
    (:OnCompleted
      _)
    (:OnBlendOut
      _)
    (:OnInterrupted
      _))
  (CallFunction|Unfreeze))

(event EventChangeSoulState
  (params (New%20Soul%20State :type E_SoulStates%20Enum :default "NewEnumerator0"))
  ;[0.8184 0.3355 1 1 40] Soul State Change
  (Variables|Default|SetSoul%20State New%20Soul%20State))

(event EventAbsorption
  (bind _bpc_combat (Variables|Default|GetBpC_Combat))
  ;[0.8184 0.3355 1 1 40] Soul Absorption
  (Animation|Montage|PlayMontage (Variables|Character|GetMesh) "/Game/Characters/Player/Animations/Absorb_Magic_Montage.Absorb_Magic_Montage" 1.5
    (:then
      (if (< (Variables|/Game/Components/BpC_Combat.BpC_Combat_C|GetHealth _bpc_combat) (Variables|/Game/Components/BpC_Combat.BpC_Combat_C|GetMax%20Health _bpc_combat))
        (Default|Heal _bpc_combat 1e+01)
        (else
          (Default|ModifyStability (Variables|Default|GetBPC_Soul) 25.0 true))))))

(event Input|KeyboardEvents|1
  (params (Key :type Key%20Structure :default "None"))
  ;[1 1 1 1 40] Time DEBUG
  (:Pressed
    (Utilities|Time|SetGlobalTimeDilation 0.25))
  (:Released
    (Utilities|Time|SetGlobalTimeDilation 1.0)))

(event Input|KeyboardEvents|C
  (params (Key :type Key%20Structure :default "None"))
  ;[0.349 0 0 1 74] Experimental
  (:Pressed
    (Utilities|FlowControl|FlipFlop
      (:A
        (Variables|Default|SetCurrentState "NewEnumerator9"))
      (:B
        (Variables|Default|SetCurrentState "NewEnumerator0")))))

(fn ConstructionScript
  (bind _bpc_combat (Variables|Default|GetBpC_Combat))
  (bind _bpc_soul (Variables|Default|GetBPC_Soul))
  (bind _bpc_combat_2 (Variables|Default|GetBpC_Combat))
  (Components|SkinnedMesh|SetLeaderPoseComponent (Variables|Default|GetHead) (Variables|Character|GetMesh) false false)
  (bind _output_get (Variables|/Game/Components/BpC_Combat.BpC_Combat_C|SetMax%20Health _bpc_combat 1e+02))
  (Variables|/Game/Components/BpC_Combat.BpC_Combat_C|SetHealth _bpc_combat _output_get)
  (Variables|/Game/Components/BPC_Soul.BPC_Soul_C|SetSoulStability _bpc_soul (Variables|/Game/Components/BPC_Soul.BPC_Soul_C|GetMaxSoulStability _bpc_soul))
  (Variables|/Game/Components/BpC_Combat.BpC_Combat_C|SetTeam%20number _bpc_combat_2 0)
  (Transformation|AttachComponentToComponent (Variables|Default|GetCast%20point) (Variables|Character|GetMesh) "DEF-HAND_L" "KeepRelative" "KeepRelative" "KeepRelative" true)
  (EventDispatchers|BindEventtoMeleeHit _bpc_combat_2 (EventDispatchers|CreateEvent :!event Custom|On%20Melee%20Hit)))

(fn EngageLock
  (bind _returnvalue (Transformation|GetActorLocation))
  (bind _charactermovement (Variables|Character|GetCharacterMovement))
  (Variables|Lock|SetCamera%20Previous%20rotation (Transformation|GetWorldRotation (Variables|Default|GetCamera)))
  (Variables|Lock|SetLock%20Distance 1e+04)
  (bind (_outhits _returnvalue_2) (Collision|MultiSphereTraceForObjects _returnvalue _returnvalue 4.5e+02 (Utilities|Array|MakeArray "ObjectTypeQuery3") false 0 "ForDuration"))
  (for _array_element _outhits
    (if _returnvalue_2
      (LocalVariables|SetFound%20Something _returnvalue_2)))
  (if (LocalVariables|GetFound%20Something)
    (Variables|Lock|SetLocked%20actor (.HitActor (Collision|BreakHitResult _array_element)))
    (Variables|Lock|SetLocked%20 true)
    (Variables|/Script/Engine.CharacterMovementComponent|SetMaxWalkSpeed _charactermovement 2.5e+02)
    (Variables|/Script/Engine.CharacterMovementComponent|SetbOrientRotationToMovement _charactermovement false)
    (Input|SetIgnoreLookInput (Game|GetPlayerController 0) true)
    (bind _returnvalue_3 (Utilities|Time|SetTimerbyFunctionName 0 "Lock too far" 0.15 true))
    (Variables|Lock|SetBreak%20Lock%20Timer _returnvalue_3)
    (Variables|Default|SetbUseControllerRotationYaw false)))

(fn LockTooFar
  (Variables|Lock|GetLocked%20actor
    (:then
      (if (> (Math|Vector|Distance(Vector) (Transformation|GetActorLocation (Variables|Lock|GetLocked%20actor)) (Transformation|GetActorLocation)) 1.2e+03)
        (CallFunction|DisengageLock)))
    (:else)))

(fn DisengageLock
  (bind _charactermovement (Variables|Character|GetCharacterMovement))
  (Transformation|SetWorldRotation (Variables|Default|GetCamera) (Variables|Lock|GetCamera%20Previous%20rotation) false false)
  (Variables|Lock|SetLocked%20actor 0)
  (Variables|Lock|SetLocked%20 false)
  (Variables|/Script/Engine.CharacterMovementComponent|SetMaxWalkSpeed _charactermovement 5e+02)
  (Variables|/Script/Engine.CharacterMovementComponent|SetbOrientRotationToMovement _charactermovement true)
  (Utilities|Time|ClearandInvalidateTimerbyHandle (Variables|Lock|GetBreak%20Lock%20Timer))
  (Input|SetIgnoreLookInput (Game|GetPlayerController 0) false)
  (Variables|Default|SetbUseControllerRotationYaw false)
  (Variables|/Script/Engine.SpringArmComponent|SetTargetArmLength (Variables|Default|GetSpringArm) (Variables|Lock|GetDefault%20Arm%20Length)))

(fn CheckDashDirection
  (bind _returnvalue (Class|Pawn|GetLastMovementInputVector))
  (bind _returnvalue_2 (Transformation|GetActorTransform))
  (bind _returnvalue_3 (Math|Vector|Normalize _returnvalue))
  (bind _returnvalue_4 (Math|Transform|InverseTransformDirection _returnvalue_2 _returnvalue_3))
  ;[1 1 1] Right
  (if (> (.y _returnvalue_4) 0.5)
    (Variables|Default|SetDashDirection 3)
    (return)
    (else
      ;[1 1 1] Left
      (if (< (.y _returnvalue_4) -0.5)
        (Variables|Default|SetDashDirection 2)
        (return)
        (else
          ;[1 1 1] Front
          (if (> (.x _returnvalue_4) 0.5)
            (Variables|Default|SetDashDirection 0)
            (return)
            (else
              ;[1 1 1] Back
              (if (< (.x _returnvalue_4) -0.5)
                (Variables|Default|SetDashDirection 1)
                (return)))))))))

(fn DashDistance
  (bind _returnvalue (Transformation|GetActorForwardVector))
  (bind _returnvalue_2 (Class|Pawn|GetLastMovementInputVector))
  (bind _returnvalue_3 (Transformation|GetActorLocation))
  (bind _maxdashdistance (Variables|Default|GetMaxDashDistance))
  (bind _returnvalue_4 (Utilities|Operators|EqualEqual :A _returnvalue_2))
  (bind _returnvalue_5 (Math|Vector|SelectVector _returnvalue _returnvalue_2 _returnvalue_4))
  (bind _returnvalue_6 (* _returnvalue_5 _maxdashdistance))
  (return (Math|Vector|SelectVector (- _returnvalue_3 _returnvalue_6) (+ _returnvalue_3 _returnvalue_6) (and _returnvalue_4 (Variables|Lock|GetLocked%20)))))

(fn SetActiveSpell
  (Variables|/Game/Components/BPC_Spells.BPC_Spells_C|SetActive%20Spell (Variables|Default|GetBPC_Spells) (Variables|Default|GetActive%20Spell)))

(fn CheckAbsorbing
  (return (Utilities|Enum|Equal(Enum) (Variables|Default|GetCurrentState) "NewEnumerator8")))

(fn GetSoulComp
  (return (Variables|Default|GetBPC_Soul)))

(fn GetActiveSpell
  (return (Variables|Default|GetActive%20Spell)))

(fn GetActiveTarget
  (return (Variables|Lock|GetLocked%20actor)))

(fn GetCameraComponent
  (return (Variables|Default|GetCamera) (Variables|Default|GetCast%20point)))

(fn GetCapsulle
  (return (Variables|Collision|GetCapsuleComponent)))

(fn GetMovementComp
  (return (Variables|Character|GetCharacterMovement)))

(fn GetSpellComp
  (return (Variables|Default|GetBPC_Spells)))

(fn GetTeamNumber
  (return (Variables|/Game/Components/BpC_Combat.BpC_Combat_C|GetTeam%20number (Variables|Default|GetBpC_Combat))))

(fn GetSoulState
  (return "NewEnumerator0"))

(fn GetCombatComp
  (return (Variables|Default|GetBpC_Combat)))

(fn GetMesh
  (return (Variables|Character|GetMesh)))

(fn Heal
  (params (Heal%20Amount :type Float%20%28double-precision%29))
  (Default|Heal (Variables|Default|GetBpC_Combat) Heal%20Amount)
  (return false))

(fn ReceiveDamage
  (params (DamageAmount :type Float%20%28double-precision%29) (Damage%20Causer :type Actor%20Object%20Reference) (Damage%20Type :type E_DamageTypes%20Enum :default "NewEnumerator6") (Damage%20Info :type S%20Damage%20Info%20Structure))
  (bind _should_react (Default|DamageReceived (Variables|Default|GetBpC_Combat) Damage%20Causer (select (Utilities|Enum|Equal(Enum) Damage%20Type "NewEnumerator7") DamageAmount (Utilities|Select :Index (Variables|Default|GetSoul%20State) :NewEnumerator0 DamageAmount :NewEnumerator1 (* DamageAmount 1.5) :NewEnumerator2 (* DamageAmount 2.0))) Damage%20Type Damage%20Info))
  (return _should_react))

(fn Stun
  (return false))