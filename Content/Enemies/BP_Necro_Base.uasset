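; BP_Necro_Base is an enemy base Blueprint driven by AIC_Necro, with montage-based attacks, step-back and hit reactions that set AI state.
; BpCCombat supplies health and a breakable state, with hit delegates bound in construction.
; Breaking starts a timed recovery; repeated hits trigger an immune death montage that spawns a soul orb on notify, while SpellDeath kills only broken enemies.
; Tick prints debug health and broken state; Die only prints.
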(event Custom|Restore
  (bind _bpc_combat (Variables|Default|GetBpC_Combat))
  ;[1 1 1 1 50] Break and Death
  (Variables|/Game/Components/BpC_Combat.BpC_Combat_C|SetHealth _bpc_combat 5e+01)
  (Default|SetStateasPassive (Variables|Default|GetAIC))
  (Variables|/Game/Components/BpC_Combat.BpC_Combat_C|SetBroken _bpc_combat false)
  (Variables|Default|SetBreakHitCount 0))

(event Custom|Spawn%20soul
  (bind _returnvalue (Transformation|GetActorTransform))
  ;[1 1 1] Spawn Magic
  (Game|SpawnActorfromClass "/Game/Enemies/BP_SoulOrb.BP_SoulOrb_C" (Math|Transform|MakeTransform (Transformation|GetSocketLocation (Variables|Character|GetMesh) "DEF-CHEST") (.rotation _returnvalue) (.scale _returnvalue)) "Undefined" "MultiplyWithRoot" 0 0))

(event Custom|Spell%20Death
  ;[1 1 1 1 50] Break and Death
  (if (Variables|/Game/Components/BpC_Combat.BpC_Combat_C|GetBroken (Variables|Default|GetBpC_Combat))
    (Animation|Montage|PlayMontage (Variables|Character|GetMesh) "/Game/Enemies/Necro_Ghoul/Ghoul_Death2_Montage.Ghoul_Death2_Montage"
      (:OnBlendOut
        (Actor|DestroyActor)))))

(event Custom|HitCount
  (bind _recover_timer (Variables|Default|GetRecover%20Timer))
  ;[1 1 1 1 50] Break and Death
  (if (>= (Variables|Default|GetBreakHitCount) 2)
    (if (Utilities|Time|IsValidTimerHandle _recover_timer)
      (Utilities|Time|ClearandInvalidateTimerbyHandle _recover_timer))
    (Variables|/Game/Components/BpC_Combat.BpC_Combat_C|SetImmune (Variables|Default|GetBpC_Combat) true)
    (bind _notifyname (Animation|Montage|PlayMontage (Variables|Character|GetMesh) "/Game/Enemies/Necro_Ghoul/Ghoul_Death_Montage.Ghoul_Death_Montage")
      (:OnBlendOut
        (Actor|DestroyActor))
      (:OnNotifyBegin
        (switch name _notifyname
          (:Spawn
            (CallFunction|SpawnSoul)))))
    (else
      (Math|Integer|IncrementInt (Variables|Default|GetBreakHitCount)
        (:%20%20
          (Animation|Montage|PlayMontage (Variables|Character|GetMesh) "/Game/Enemies/Necro_Ghoul/NG_Hit.NG_Hit"))))))

(event EventBeginPlay
  ;[1 1 1] Start
  (bind _asaic_necro (Utilities|Casting|CastToAIC_Necro (AI|GetAIController self)))
  (Variables|Default|SetAIC _asaic_necro))

(event Collision|EventActorBeginOverlap
  (params (OtherActor :type Actor%20Object%20Reference)))

(event EventBreak
  ;[1 1 1 1 50] Break and Death
  (Default|SetStateasBroken (Variables|Default|GetAIC))
  (bind _returnvalue (Utilities|Time|SetTimerbyEvent (delegate Custom|Restore) 1e+01))
  (Variables|Default|SetRecover%20Timer _returnvalue)
  (Animation|Montage|PlayMontage (Variables|Character|GetMesh) "/Game/Enemies/Necro_Ghoul/NG_Hit.NG_Hit"))

(event EventDie
  (params (Spell? :type Boolean) (Killer :type Actor%20Object%20Reference))
  ;[1 1 1 1 50] Break and Death
  (Development|PrintString "dead call"))

(event EventAttack
  ;[1 1 1] Attack
  (Animation|Montage|PlayMontage (Variables|Character|GetMesh) (.OutItem (Utilities|Array|Random (Variables|/Game/Enemies/Data_Assets/DA_EnemyBase.DA_EnemyBase_C|GetATK_montages (Variables|Default|GetData%20Asset))))
    (:OnCompleted
      _)
    (:OnBlendOut
      _)
    (:OnInterrupted
      _))
  (Default|CallOnAttackEnd))

(event EventStepBack
  ;[1 1 1] Evade
  (Animation|Montage|PlayMontage (Variables|Character|GetMesh) "/Game/Enemies/Necro_Ghoul/NG_Stepback.NG_Stepback"))

(event EventDamageReaction
  (params (Damage%20Causer :type Actor%20Object%20Reference) (Damage%20Type :type E_DamageTypes%20Enum :default "NewEnumerator6"))
  (bind _aic (Variables|Default|GetAIC))
  ;[1 1 1] Receive damage
  (Default|SetStateasFrozen (Variables|Default|GetAIC))
  (Animation|Montage|PlayMontage (Variables|Character|GetMesh) (Variables|Default|GetHit%20Montage)
    (:OnBlendOut
      _)
    (:OnInterrupted
      _))
  (Utilities|FlowControl|Delay 0.1)
  (if (not (Variables|/Game/Components/BpC_Combat.BpC_Combat_C|GetBroken (Variables|Default|GetBpC_Combat)))
    (Utilities|IsValid _aic
      (:Is%20Valid
        (Default|SetStateasCombat _aic 0 true)))))

(event EventSpecialAttack
  ;[1 1 1] Special Attack
  (Animation|Montage|PlayMontage (Variables|Character|GetMesh) (Utilities|Array|Get(acopy) (Variables|/Game/Enemies/Data_Assets/DA_EnemyBase.DA_EnemyBase_C|GetSpecial%20Montage (Variables|Default|GetData%20Asset)))
    (:OnCompleted
      _)
    (:OnBlendOut
      _)
    (:OnInterrupted
      _))
  (Default|CallOnAttackEnd))

(event EventTick
  (params (DeltaSeconds :type Float%20%28single-precision%29))
  (bind _bpc_combat (Variables|Default|GetBpC_Combat))
  (Development|PrintString (Utilities|String|ToString(Float) (Variables|/Game/Components/BpC_Combat.BpC_Combat_C|GetHealth _bpc_combat)) true true "(R=0.000000,G=1.000000,B=0.225339,A=1.000000)" DeltaSeconds)
  (Development|PrintString (Utilities|String|ToString(Boolean) (Variables|/Game/Components/BpC_Combat.BpC_Combat_C|GetBroken _bpc_combat)) true true "(R=1.000000,G=0.146624,B=0.000000,A=1.000000)" DeltaSeconds))

(fn ConstructionScript
  (bind _bpc_combat (Variables|Default|GetBpC_Combat))
  (|CallParentFunction)
  (Variables|/Game/Components/BpC_Combat.BpC_Combat_C|SetTeam%20number _bpc_combat 1)
  (EventDispatchers|BindEventtoSpellHit _bpc_combat (EventDispatchers|CreateEvent :!event Custom|Spell%20Death))
  (Variables|/Game/Components/BpC_Combat.BpC_Combat_C|SetIsBreakable? _bpc_combat true)
  (EventDispatchers|BindEventtoOnBrokenHit _bpc_combat (EventDispatchers|CreateEvent :!event Custom|HitCount)))

(fn GetDataAsset
  (return (Variables|Default|GetData%20Asset)))

(fn GetTarget
  (return (Variables|/Game/Enemies/AI/AIC_Necro.AIC_Necro_C|GetAttack%20Target (Variables|Default|GetAIC))))