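; BP_Dummy is a combat dummy enemy that receives damage and plays a hit reaction.
; Its damage, team number and combat component functions route to BpCCombat, while Heal and Stun return false and the active-target getter returns nothing.
; DamageReaction prints a debug string and plays a montage on the mesh, then triggers a hitstop through the combat component after a short delay.
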(event EventBeginPlay)

(event Collision|EventActorBeginOverlap
  (params (OtherActor :type Actor%20Object%20Reference)))

(event EventTick
  (params (DeltaSeconds :type Float%20%28single-precision%29)))

(event EventDamageReaction
  (params (Damage%20Causer :type Actor%20Object%20Reference) (Damage%20Type :type E_DamageTypes%20Enum :default "NewEnumerator6"))
  (Development|PrintString "Hello")
  (Animation|Montage|PlayMontage (Variables|Character|GetMesh) "/Game/Enemies/Dummy/Dummy_Anim_Montage.Dummy_Anim_Montage" 1.5
    (:then
      (Utilities|FlowControl|Delay 0.1)
      (Default|Hitstop (Variables|Default|GetBpC_Combat) self))))

(fn ConstructionScript)

(fn GetActiveTarget
  (return 0))

(fn GetTeamNumber
  (return (Variables|/Game/Components/BpC_Combat.BpC_Combat_C|GetTeam%20number (Variables|Default|GetBpC_Combat))))

(fn GetCombatComp
  (return (Variables|Default|GetBpC_Combat)))

(fn Heal
  (params (Heal%20Amount :type Float%20%28double-precision%29))
  (return false))

(fn ReceiveDamage
  (params (Damage%20Causer :type Actor%20Object%20Reference) (Damage%20Info :type S%20Damage%20Info%20Structure))
  (bind _should_react (Default|DamageReceived (Variables|Default|GetBpC_Combat) Damage%20Causer Damage%20Info))
  (return _should_react))

(fn Stun
  (return false))