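; BPC_Spells is an actor component that stores spells and modifiers per slot and casts them for its owner.
; CastSpell routes by type: bursts spawn at the owner, area spells trace aim on a timer until EndSpell places them, ranged spells fire at the target or camera trace.
; Modifiers reshape ranged casts into cone, line or circle volleys or timer-driven full-auto.
; Casts drain the owner's soul stability through message calls.
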(event Custom|Barrage
  (params (Spell%20casted :type PDA%20Spell%20Base%20Object%20Reference) (Projs :type Integer))
  (for _index (range 0 Projs)
    (Utilities|FlowControl|Delay (* 1.0 _index))
    (CallFunction|HandleRanged Spell%20casted)
    (Class|BPISoulActor|ModifySoulStablity(Message) (Components|GetOwner) (Variables|/Game/Spells/Spell_Data_Assets/PDA_SpellBase.PDA_SpellBase_C|GetStability%20Cost Spell%20casted) true)))

(event Custom|FullAuto
  (CallFunction|HandleRanged (stale Custom|Full%20Auto%20start Spell%20being%20casted)))

(event Custom|Full%20Auto%20start
  (params (Spell%20being%20casted :type PDA%20Spell%20Base%20Object%20Reference))
  (bind _returnvalue (Utilities|Time|SetTimerbyEvent (delegate Custom|FullAuto) 0.1 true))
  (Variables|Default|SetFull%20Auto%20Timer _returnvalue))

(event Custom|Clear%20Damaged
  (Utilities|FlowControl|DelayUntilNextTick)
  (Utilities|Array|Clear (Variables|Default|GetDamaged%20Actors)))

(event EventBeginPlay)

(fn CastSpell
  (params (Spell%20Slot :type E_SpellSlot%20Enum :default "NewEnumerator0"))
  (bind _equiped_spells (Variables|Default|GetEquiped%20Spells))
  (bind _equiped_modifiers (Variables|Default|GetEquiped%20Modifiers))
  (bind (_value _returnvalue) (Utilities|Map|Find _equiped_spells Spell%20Slot))
  (bind (_value_2 _returnvalue_2) (Utilities|Map|Find _equiped_modifiers Spell%20Slot))
  (bind _spell_type (Variables|/Game/Spells/Spell_Data_Assets/PDA_SpellBase.PDA_SpellBase_C|GetSpell%20Type _value))
  ;[0.224 0.003307 0] Start
  (if _returnvalue
    ;[0.224 0.003307 0] Check for modifier
    (if _returnvalue_2
      ;[1 1 1] Modified Cast
      (switch Utilities|FlowControl|Switch|SwitchonE_SpellTypes _spell_type
        (:NewEnumerator0
          (CallFunction|HandleBurstModified _value _value_2))
        (:NewEnumerator4
          (CallFunction|HandleRangedModified _value _value_2)))
      (Development|PrintString "cast modified spell")
      (else
        ;[1 1 1] Raw Cast
        (switch Utilities|FlowControl|Switch|SwitchonE_SpellTypes _spell_type
          (:NewEnumerator0
            (CallFunction|HandleBurst _value))
          (:NewEnumerator1
            (Area|StartAreaTrace))
          (:NewEnumerator4
            (CallFunction|HandleRanged _value)))))))

(fn EndSpell
  (params (Slot :type E_SpellSlot%20Enum :default "NewEnumerator0"))
  (bind _equiped_spells (Variables|Default|GetEquiped%20Spells))
  (bind _full_auto_timer (Variables|Default|GetFull%20Auto%20Timer))
  (bind (_value _returnvalue) (Utilities|Map|Find _equiped_spells Slot))
  (if _returnvalue
    (switch Utilities|FlowControl|Switch|SwitchonE_SpellTypes (Variables|/Game/Spells/Spell_Data_Assets/PDA_SpellBase.PDA_SpellBase_C|GetSpell%20Type _value)
      (:NewEnumerator1
        (bind _outputpin (CallFunction|HandleArea _value))
        (if _outputpin
          (CallFunction|ConsumeStability (Variables|/Game/Spells/Spell_Data_Assets/PDA_SpellBase.PDA_SpellBase_C|GetStability%20Cost _value) false)
          (Variables|Default|SetArea%20Location "0, 0, 0")))
      (:NewEnumerator4
        (if (Utilities|Time|IsValidTimerHandle _full_auto_timer)
          (Utilities|Time|ClearandInvalidateTimerbyHandle _full_auto_timer))))))

(fn HandleBurst
  (params (Spell%20Being%20Casted :type PDA%20Spell%20Base%20Object%20Reference))
  (bind _returnvalue (Components|GetOwner))
  (Game|SpawnActorfromClass (Variables|/Game/Spells/Spell_Data_Assets/PDA_SpellBase.PDA_SpellBase_C|GetSpell%20Class Spell%20Being%20Casted) (Math|Transform|MakeTransform (Transformation|GetActorLocation _returnvalue) (Transformation|GetActorRotation _returnvalue) "1.000000,1.000000,1.000000") "Undefined" "MultiplyWithRoot" 0 _returnvalue Spell%20Being%20Casted "0.000000,0.000000,0.000000" 0 0)
  (CallFunction|ConsumeStability (Variables|/Game/Spells/Spell_Data_Assets/PDA_SpellBase.PDA_SpellBase_C|GetStability%20Cost Spell%20Being%20Casted) false))

(fn HandleArea
  (params (Spell%20Being%20Casted :type PDA%20Spell%20Base%20Object%20Reference))
  (bind _current_target (Class|BPIDamageable|GetActiveTarget(Message) (Components|GetOwner)))
  (Utilities|IsValid _current_target
    (:Is%20Valid
      (Variables|Default|SetArea%20Location (Transformation|GetActorLocation _current_target))
      (Game|SpawnActorfromClass (Variables|/Game/Spells/Spell_Data_Assets/PDA_SpellBase.PDA_SpellBase_C|GetSpell%20Class Spell%20Being%20Casted) (Math|Transform|MakeTransform (Variables|Default|GetArea%20Location) "0, 0, 0" "1.000000,1.000000,1.000000") "Undefined" "MultiplyWithRoot" 0 (Components|GetOwner) (LocalVariables|GetSpell%20being%20casted) "0.000000,0.000000,0.000000" 0 0 :!label _label))
    (:Is%20Not%20Valid
      (if (Utilities|Operators|NotEqual(!=) :A (Variables|Default|GetArea%20Location))
        (goto _label)
        (else
          _))))
  (Utilities|Time|ClearandInvalidateTimerbyHandle (Variables|Default|GetArea%20Trace%20Timer))
  (return (Utilities|Operators|NotEqual(!=) :A (Variables|Default|GetArea%20Location))))

(fn StartAreaTrace
  (bind _returnvalue (Utilities|Time|SetTimerbyFunctionName 0 "Area aim trace" 0.1 true))
  (Variables|Default|SetArea%20Trace%20Timer _returnvalue)
  (Default|CallAllowRelease))

(fn HandleRanged
  (params (Spell%20being%20casted :type PDA%20Spell%20Base%20Object%20Reference))
  (bind _returnvalue (Components|GetOwner))
  (bind _returnvalue_2 (Components|GetOwner))
  (bind _returnvalue_3 (Components|GetOwner))
  (bind _full_auto_timer (Variables|Default|GetFull%20Auto%20Timer))
  (bind _full_auto_timer_2 (Variables|Default|GetFull%20Auto%20Timer))
  (bind _returnvalue_4 (Utilities|Time|IsValidTimerHandle _full_auto_timer_2))
  (bind _returnvalue_5 (Utilities|Time|IsValidTimerHandle _full_auto_timer))
  (bind _stability_cost (Variables|/Game/Spells/Spell_Data_Assets/PDA_SpellBase.PDA_SpellBase_C|GetStability%20Cost Spell%20being%20casted))
  (bind _stability_cost_2 (Variables|/Game/Spells/Spell_Data_Assets/PDA_SpellBase.PDA_SpellBase_C|GetStability%20Cost Spell%20being%20casted))
  ;[1 1 1] Check target and origin
  (bind _newparam (Class|BPIComponentExtractor|GetCameraComponent(Message) _returnvalue))
  (bind _current_target (Class|BPIDamageable|GetActiveTarget(Message) _returnvalue))
  (LocalVariables|SetOrigin (Transformation|GetWorldLocation _newparam))
  (LocalVariables|SetForward%20vector (Transformation|GetActorForwardVector _returnvalue))
  (Utilities|IsValid _current_target
    (:Is%20Valid
      ;[0.8234 1 0.7067 1 90] With target
      (LocalVariables|SetDirection (- (Transformation|GetActorLocation _current_target) (LocalVariables|GetOrigin)))
      (bind _returnvalue_6 (Game|SpawnActorfromClass (Variables|/Game/Spells/Spell_Data_Assets/PDA_SpellBase.PDA_SpellBase_C|GetSpell%20Class Spell%20being%20casted) (Math|Transform|MakeTransform (+ (LocalVariables|GetOrigin) (* (LocalVariables|GetForward%20vector) 1e+01)) (Math|Rotator|MakeRotfromX (LocalVariables|GetDirection)) "1.000000,1.000000,1.000000") "Undefined" "MultiplyWithRoot" 0 (Components|GetOwner) Spell%20being%20casted (Math|Vector|Normalize (LocalVariables|GetDirection)) 0 0))
      (bind _caps (Class|BPIComponentExtractor|GetCapsulle(Message) _returnvalue_3))
      (Collision|IgnoreActorwhenMoving _caps _returnvalue_6 true)
      (Collision|IgnoreActorwhenMoving (Variables|/Game/Spells/Actors/BPA_Spell_Master.BPA_Spell_Master_C|GetRootBox _returnvalue_6) _returnvalue_3 true)
      (CallFunction|ConsumeStability (select _returnvalue_4 (* _stability_cost 0.1) _stability_cost) _returnvalue_4))
    (:Is%20Not%20Valid
      ;[0.4463 0.9602 1 1 74] Without target
      (bind (_camera _newparam_2) (Class|BPIComponentExtractor|GetCameraComponent(Message) (Components|GetOwner)))
      (bind (_outhit _returnvalue_7) (Collision|LineTraceForObjects (Transformation|GetWorldLocation _camera) (+ (Transformation|GetWorldLocation _camera) (* (Math|Vector|GetForwardVector _camera) 5e+03)) (Utilities|Array|MakeArray "ObjectTypeQuery1" "ObjectTypeQuery2" "ObjectTypeQuery3") false 0 "ForDuration"))
      (Utilities|FlowControl|Sequence
        (:then_0
          (bind _aspawn (Utilities|Casting|CastToPawn _returnvalue_2))
          (bind _returnvalue_8 (Game|SpawnActorfromClass (Variables|/Game/Spells/Spell_Data_Assets/PDA_SpellBase.PDA_SpellBase_C|GetSpell%20Class Spell%20being%20casted) (Math|Transform|MakeTransform (Transformation|GetWorldLocation _newparam_2) (Math|Rotator|MakeRotfromX (Math|Vector|Normalize (- (Math|Vector|SelectVector (.Location (Collision|BreakHitResult _outhit)) (.TraceEnd (Collision|BreakHitResult _outhit)) _returnvalue_7) (Transformation|GetWorldLocation _newparam_2))))) "Undefined" "MultiplyWithRoot" _aspawn _returnvalue_2 Spell%20being%20casted (Math|Vector|Normalize (- (Math|Vector|SelectVector (.Location (Collision|BreakHitResult _outhit)) (.TraceEnd (Collision|BreakHitResult _outhit)) _returnvalue_7) (Transformation|GetWorldLocation _newparam_2))) 0 _aspawn))
          (bind _caps_2 (Class|BPIComponentExtractor|GetCapsulle(Message) _returnvalue_2))
          (Collision|IgnoreActorwhenMoving _caps_2 _returnvalue_8 true)
          (Collision|IgnoreActorwhenMoving (Variables|/Game/Spells/Actors/BPA_Spell_Master.BPA_Spell_Master_C|GetRootBox _returnvalue_8) (Components|GetOwner) true)
          (CallFunction|ConsumeStability (select _returnvalue_5 (* _stability_cost_2 0.1) _stability_cost_2) _returnvalue_5))
        (:then_1
          (Development|PrintString (Utilities|GetDisplayName (.HitComponent (Collision|BreakHitResult _outhit)))))))))

(fn ConeCheck
  (params (Start :type Vector) (forward :type Vector) (Radius :type Float%20%28single-precision%29) (Spread%20Angle :type Float%20%28double-precision%29))
  (bind _outhits (Collision|MultiSphereTraceForObjects Start Start Radius (Utilities|Array|MakeArray "ObjectTypeQuery3") false 0 "ForOneFrame"))
  (for _array_element _outhits
    (if (>= (Math|Vector|DotProduct forward (Math|Vector|Normalize (- (Transformation|GetActorLocation (.HitActor (Collision|BreakHitResult _array_element))) Start))) (Math|Trig|Cos(Radians) (Math|Trig|DegreesToRadians (/ Spread%20Angle 2.0))))
      _)))

(fn CancelAreaTrace
  (Utilities|Time|ClearandInvalidateTimerbyHandle (Variables|Default|GetArea%20Trace%20Timer)))

(fn AreaAimTrace
  (bind _camera (Class|BPIComponentExtractor|GetCameraComponent(Message) (Components|GetOwner)))
  (bind (_outhit _returnvalue) (Collision|LineTraceByChannel (Transformation|GetWorldLocation _camera) (+ (Transformation|GetWorldLocation _camera) (* (Math|Vector|GetForwardVector _camera) 2.5e+03)) "TraceTypeQuery1" false 0 "ForDuration"))
  (if _returnvalue
    (Rendering|Debug|DrawDebugSphere (.Location (Collision|BreakHitResult _outhit)) 1e+01 12 "(R=1.000000,G=1.000000,B=1.000000,A=1.000000)" 1.0)
    (Variables|Default|SetArea%20Location (.Location (Collision|BreakHitResult _outhit)))
    (else
      (Variables|Default|SetArea%20Location "0, 0, 0"))))

(fn EquipSpell
  (params (Slot :type E_SpellSlot%20Enum :default "NewEnumerator0") (Spell :type PDA%20Spell%20Base%20Object%20Reference))
  (Utilities|Map|Add (Variables|Default|GetEquiped%20Spells) Slot Spell))

(fn ConsumeStability
  (params (Stability%20Amount :type Float%20%28double-precision%29) (Modified :type Boolean))
  (Class|BPISoulActor|ModifySoulStablity(Message) (Components|GetOwner) (Math|Float|SelectFloat (* Stability%20Amount 1.5) Stability%20Amount Modified) false)
  (Default|CallSpellCasted 0.0))

(fn EquipModifier
  (params (Slot :type E_SpellSlot%20Enum :default "NewEnumerator0") (Spell :type PDA%20Spell%20Base%20Object%20Reference))
  (bind _equiped_spells (Variables|Default|GetEquiped%20Spells))
  (bind (_value _returnvalue) (Utilities|Map|Find _equiped_spells Slot))
  (if _returnvalue
    (if (Variables|/Game/Spells/Spell_Data_Assets/PDA_SpellBase.PDA_SpellBase_C|GetIs%20modifiable _value)
      (Utilities|Map|Add (Variables|Default|GetEquiped%20Modifiers) Slot Spell)
      (Development|PrintString "modifier added" true true "(R=1.000000,G=0.179098,B=0.000000,A=1.000000)"))
    (else
      (Development|PrintString "no spell in slot" true true "(R=1.000000,G=0.137598,B=0.000000,A=1.000000)"))))

(fn HandleRangedModified
  (params (Spell%20being%20casted :type PDA%20Spell%20Base%20Object%20Reference) (Modifier :type PDA%20Spell%20Base%20Object%20Reference))
  (bind _returnvalue (Components|GetOwner))
  (bind _returnvalue_2 (Components|GetOwner))
  ;[1 1 1] Check target and origin
  (bind _newparam (Class|BPIComponentExtractor|GetCameraComponent(Message) _returnvalue))
  (bind _current_target (Class|BPIDamageable|GetActiveTarget(Message) _returnvalue))
  (LocalVariables|SetOrigin (Transformation|GetWorldLocation _newparam))
  (LocalVariables|SetForward%20vector (Transformation|GetActorForwardVector _returnvalue))
  (Utilities|IsValid _current_target
    (:Is%20Valid
      (LocalVariables|SetDirection (- (Transformation|GetActorLocation _current_target) (LocalVariables|GetOrigin)))
      (switch Utilities|FlowControl|Switch|SwitchonE_SpellTypes (Variables|/Game/Spells/Spell_Data_Assets/PDA_SpellBase.PDA_SpellBase_C|GetSpell%20Type Modifier) :!label _label
        (:NewEnumerator0
          (bind _aspda_burst_spell (Utilities|Casting|CastToPDA_Burst_Spell Modifier))
          (switch Utilities|FlowControl|Switch|SwitchonE_ShapeType (Variables|/Game/Spells/Spell_Data_Assets/PDA_Burst_Spell.PDA_Burst_Spell_C|GetBurst%20Shape _aspda_burst_spell)
            (:NewEnumerator0
              (LocalVariables|SetProjectile%20count (/ (Math|Float|Truncate (Variables|/Game/Spells/Spell_Data_Assets/PDA_Burst_Spell.PDA_Burst_Spell_C|GetSpread%20Angle _aspda_burst_spell)) 10))
              (LocalVariables|SetAngle (Variables|/Game/Spells/Spell_Data_Assets/PDA_Burst_Spell.PDA_Burst_Spell_C|GetSpread%20Angle _aspda_burst_spell))
              ;[1 1 1] alpha
              (for _index (range 0 (- (LocalVariables|GetProjectile%20count) 1)) :!label _label_2
                (bind _returnvalue_3 (Game|SpawnActorfromClass (Variables|/Game/Spells/Spell_Data_Assets/PDA_SpellBase.PDA_SpellBase_C|GetSpell%20Class Spell%20being%20casted) (Math|Transform|MakeTransform (Utilities|Select :Index (stale _index_2) :Option%200 (LocalVariables|GetOrigin) :Option%201 (+ (LocalVariables|GetOrigin) "20.000000,0.000000,20.000000") :Option%202 (+ (LocalVariables|GetOrigin) "-20.000000,0.000000,20.000000")) "0, 0, 0" "1.000000,1.000000,1.000000") "Undefined" "MultiplyWithRoot" 0 (Components|GetOwner) Spell%20being%20casted (Math|Vector|RotateVectorAroundAxis (LocalVariables|GetForward%20Vector) (Math|Float|Lerp (* (/ (LocalVariables|GetAngle) 2.0) -1.0) (/ (LocalVariables|GetAngle) 2.0) (/ (Math|Conversions|ToFloat(Integer) _index) (- (Math|Conversions|ToFloat(Integer) (LocalVariables|GetProjectile%20count)) 1.0))) (Transformation|GetActorUpVector (Components|GetOwner))) Modifier 0))
                (bind _caps (Class|BPIComponentExtractor|GetCapsulle(Message) _returnvalue_2))
                (Collision|IgnoreActorwhenMoving _caps _returnvalue_3 true)
                (Collision|IgnoreActorwhenMoving (Variables|/Game/Spells/Actors/BPA_Spell_Master.BPA_Spell_Master_C|GetRootBox _returnvalue_3) _returnvalue_2 true)
                (CallFunction|ConsumeStability (Variables|/Game/Spells/Spell_Data_Assets/PDA_SpellBase.PDA_SpellBase_C|GetStability%20Cost Spell%20being%20casted) true)))
            (:NewEnumerator1
              (LocalVariables|SetProjectile%20count (/ (/ (Math|Float|Truncate (Variables|/Game/Spells/Spell_Data_Assets/PDA_Burst_Spell.PDA_Burst_Spell_C|GetSpread%20Angle _aspda_burst_spell)) 10) 2))
              (LocalVariables|SetAngle 0.0)
              (LocalVariables|SetForward%20vector (LocalVariables|GetDirection))
              (for _index_2 (range 0 (LocalVariables|GetProjectile%20count))
                (bind _returnvalue_4 (Game|SpawnActorfromClass (Variables|/Game/Spells/Spell_Data_Assets/PDA_SpellBase.PDA_SpellBase_C|GetSpell%20Class Spell%20being%20casted) (Math|Transform|MakeTransform (Utilities|Select :Index _index_2 :Option%200 (LocalVariables|GetOrigin) :Option%201 (+ (LocalVariables|GetOrigin) "20.000000,0.000000,20.000000") :Option%202 (+ (LocalVariables|GetOrigin) "-20.000000,0.000000,20.000000")) "0, 0, 0" "1.000000,1.000000,1.000000") "Undefined" "MultiplyWithRoot" 0 (Components|GetOwner) Spell%20being%20casted (Math|Vector|RotateVectorAroundAxis (LocalVariables|GetForward%20Vector) (Math|Float|Lerp (* (/ (LocalVariables|GetAngle) 2.0) -1.0) (/ (LocalVariables|GetAngle) 2.0) (/ (Math|Conversions|ToFloat(Integer) _index) (- (Math|Conversions|ToFloat(Integer) (LocalVariables|GetProjectile%20count)) 1.0))) (Transformation|GetActorUpVector (Components|GetOwner))) Modifier 0))
                (bind _caps_2 (Class|BPIComponentExtractor|GetCapsulle(Message) _returnvalue_2))
                (Collision|IgnoreActorwhenMoving _caps_2 _returnvalue_4 true)
                (Collision|IgnoreActorwhenMoving (Variables|/Game/Spells/Actors/BPA_Spell_Master.BPA_Spell_Master_C|GetRootBox _returnvalue_4) _returnvalue_2 true)
                (CallFunction|ConsumeStability (Variables|/Game/Spells/Spell_Data_Assets/PDA_SpellBase.PDA_SpellBase_C|GetStability%20Cost Spell%20being%20casted) true)))
            (:NewEnumerator2
              (LocalVariables|SetProjectile%20count (* (/ (Math|Float|Truncate (Variables|/Game/Spells/Spell_Data_Assets/PDA_Burst_Spell.PDA_Burst_Spell_C|GetSpread%20Angle _aspda_burst_spell)) 10) 2))
              (LocalVariables|SetAngle 3.6e+02)
              (goto _label_2))))
        (:NewEnumerator1
          (LocalVariables|SetForward%20vector (LocalVariables|GetDirection))
          (bind _returnvalue_5 (Game|SpawnActorfromClass (Variables|/Game/Spells/Spell_Data_Assets/PDA_SpellBase.PDA_SpellBase_C|GetSpell%20Class Spell%20being%20casted) (Math|Transform|MakeTransform (Utilities|Select :Index _index_2 :Option%200 (LocalVariables|GetOrigin) :Option%201 (+ (LocalVariables|GetOrigin) "20.000000,0.000000,20.000000") :Option%202 (+ (LocalVariables|GetOrigin) "-20.000000,0.000000,20.000000")) "0, 0, 0" "1.000000,1.000000,1.000000") "Undefined" "MultiplyWithRoot" 0 (Components|GetOwner) Spell%20being%20casted (Math|Vector|RotateVectorAroundAxis (LocalVariables|GetForward%20Vector) (Math|Float|Lerp (* (/ (LocalVariables|GetAngle) 2.0) -1.0) (/ (LocalVariables|GetAngle) 2.0) (/ (Math|Conversions|ToFloat(Integer) _index) (- (Math|Conversions|ToFloat(Integer) (LocalVariables|GetProjectile%20count)) 1.0))) (Transformation|GetActorUpVector (Components|GetOwner))) Modifier 0))
          (bind _caps_3 (Class|BPIComponentExtractor|GetCapsulle(Message) _returnvalue_2))
          (Collision|IgnoreActorwhenMoving _caps_3 _returnvalue_5 true)
          (Collision|IgnoreActorwhenMoving (Variables|/Game/Spells/Actors/BPA_Spell_Master.BPA_Spell_Master_C|GetRootBox _returnvalue_5) _returnvalue_2 true)
          (CallFunction|ConsumeStability (Variables|/Game/Spells/Spell_Data_Assets/PDA_SpellBase.PDA_SpellBase_C|GetStability%20Cost Spell%20being%20casted) true))
        (:NewEnumerator4
          (CallFunction|FullAutoStart Spell%20being%20casted))))
    (:Is%20Not%20Valid
      ;[0.4463 0.9602 1 1 74] Without target
      (bind (_camera _newparam_2) (Class|BPIComponentExtractor|GetCameraComponent(Message) (Components|GetOwner)))
      (bind (_outhit _returnvalue_6) (Collision|LineTraceForObjects (Transformation|GetWorldLocation _camera) (+ (Transformation|GetWorldLocation _camera) (* (Math|Vector|GetForwardVector _camera) 5e+03)) (Utilities|Array|MakeArray "ObjectTypeQuery1" "ObjectTypeQuery2" "ObjectTypeQuery3") false 0 "ForDuration"))
      (Utilities|FlowControl|Sequence
        (:then_0
          (LocalVariables|SetDirection (Math|Vector|Normalize (- (Math|Vector|SelectVector (.Location (Collision|BreakHitResult _outhit)) (.TraceEnd (Collision|BreakHitResult _outhit)) _returnvalue_6) (Transformation|GetWorldLocation _newparam_2))))
          (goto _label))
        (:then_1
          (Development|PrintString (Utilities|GetDisplayName (.HitComponent (Collision|BreakHitResult _outhit)))))))))

(fn HandleBurstModified
  (params (Spell%20Being%20Casted :type PDA%20Spell%20Base%20Object%20Reference) (Modifier :type PDA%20Spell%20Base%20Object%20Reference))
  (bind _returnvalue (Components|GetOwner))
  (Game|SpawnActorfromClass (Variables|/Game/Spells/Spell_Data_Assets/PDA_SpellBase.PDA_SpellBase_C|GetSpell%20Class Spell%20Being%20Casted) (Math|Transform|MakeTransform (Transformation|GetActorLocation _returnvalue) "0, 0, 0" "1.000000,1.000000,1.000000") "Undefined" "MultiplyWithRoot" 0 _returnvalue Spell%20Being%20Casted "0.000000,0.000000,0.000000" Modifier 0)
  (CallFunction|ConsumeStability (Variables|/Game/Spells/Spell_Data_Assets/PDA_SpellBase.PDA_SpellBase_C|GetStability%20Cost Spell%20Being%20Casted) false))